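; GameManager actor that handles level-wide input: pausing, restarting the level and checkpoint teleports.
; On BeginPlay it enables input, creates the WDG_Pause widget and caches the MyCharacter_Player reference.
; Pause toggles the widget, game pause and mouse cursor, while custom events switch the player's state between CINEMATIC and IDLE.
; Hardcoded AZERTY number-row keys teleport the player to the matching entry in the Checkpoints array.
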(event Custom|ResetPlayerMoves
  (params (textToPrint :type String))
  ;[1 1 1] Cinematics
  (Development|PrintString textToPrint)
  (Variables|/Script/BrawlSlash.Character_Base|Setstate (Variables|Default|GetPlayer) "IDLE"))

(event Custom|StopPlayerMoves
  (params (textToPrint :type String))
  ;[1 1 1] Cinematics
  (Development|PrintString textToPrint)
  (Variables|/Script/BrawlSlash.Character_Base|Setstate (Variables|Default|GetPlayer) "CINEMATIC"))

(event EventBeginPlay
  (bind _returnvalue (Game|GetPlayerController 0))
  ;[1 1 1] Create Pause Widget at Begin
  (Input|EnableInput _returnvalue)
  (bind _returnvalue_2 (UserInterface|CreateWidget "/Game/Blueprints/UI/WDG_Pause.WDG_Pause_C" _returnvalue))
  (Variables|Default|SetPauseMenu _returnvalue_2)
  (bind _asmy_character_player (Utilities|Casting|CastToMyCharacter_Player (Game|GetPlayerCharacter 0)))
  (Variables|Default|SetPlayer _asmy_character_player))

(event Input|ActionEvents|InputActionRestartLevel
  (params (Key :type Key%20Structure :default "None"))
  ;[1 1 1] Restart level
  (:Pressed
    (bind _returnvalue (Game|GetCurrentLevelName true))
    (Game|OpenLevel(byName) (Utilities|String|StringToName _returnvalue))))

(event Input|ActionEvents|InputActionPauseGame
  (params (Key :type Key%20Structure :default "None"))
  (:Pressed
    (if (Game|IsGamePaused)
      ;[1 1 1] Unpause
      (Widget|RemovefromParent (Variables|Default|GetPauseMenu))
      (Game|SetGamePaused false)
      (Variables|/Script/Engine.PlayerController|SetbShowMouseCursor (Game|GetPlayerController 0) false)
      (else
        ;[1 1 1] Pause
        (UserInterface|Viewport|AddtoViewport (Variables|Default|GetPauseMenu) 0)
        (Game|SetGamePaused true)
        (Variables|/Script/Engine.PlayerController|SetbShowMouseCursor (Game|GetPlayerController 0) true)))))

(event Input|KeyboardEvents|Ampersand
  (params (Key :type Key%20Structure :default "None"))
  (bind _checkpoints (Variables|Default|GetCheckpoints))
  (bind _output (Utilities|Array|Get(acopy) _checkpoints))
  ;[1 1 1] Tp on checkpoint
  (:Pressed
    (if (!= _output 0)
      (if (Utilities|IsValid _output)
        (Transformation|SetActorLocation (Variables|Default|GetPlayer) (Transformation|GetActorLocation _output) false false)))))

(event Input|KeyboardEvents|EAccentAigu
  (params (Key :type Key%20Structure :default "None"))
  (bind _checkpoints (Variables|Default|GetCheckpoints))
  (bind _output (Utilities|Array|Get(acopy) _checkpoints 1))
  ;[1 1 1] Tp on checkpoint
  (:Pressed
    (if (!= _output 0)
      (if (Utilities|IsValid _output)
        (Transformation|SetActorLocation (Variables|Default|GetPlayer) (Transformation|GetActorLocation _output) false false)))))

(event Input|KeyboardEvents|Quote
  (params (Key :type Key%20Structure :default "None"))
  (bind _checkpoints (Variables|Default|GetCheckpoints))
  (bind _output (Utilities|Array|Get(acopy) _checkpoints 2))
  ;[1 1 1] Tp on checkpoint
  (:Pressed
    (if (!= _output 0)
      (if (Utilities|IsValid _output)
        (Transformation|SetActorLocation (Variables|Default|GetPlayer) (Transformation|GetActorLocation _output) false false)))))

(event Input|KeyboardEvents|Apostrophe
  (params (Key :type Key%20Structure :default "None"))
  (bind _checkpoints (Variables|Default|GetCheckpoints))
  (bind _output (Utilities|Array|Get(acopy) _checkpoints 3))
  ;[1 1 1] Tp on checkpoint
  (:Pressed
    (if (!= _output 0)
      (if (Utilities|IsValid _output)
        (Transformation|SetActorLocation (Variables|Default|GetPlayer) (Transformation|GetActorLocation _output) false false)))))

(event Input|KeyboardEvents|LeftParantheses
  (params (Key :type Key%20Structure :default "None"))
  (bind _checkpoints (Variables|Default|GetCheckpoints))
  (bind _output (Utilities|Array|Get(acopy) _checkpoints 4))
  ;[1 1 1] Tp on checkpoint
  (:Pressed
    (if (!= _output 0)
      (if (Utilities|IsValid _output)
        (Transformation|SetActorLocation (Variables|Default|GetPlayer) (Transformation|GetActorLocation _output) false false)))))

(event Input|KeyboardEvents|RightParantheses
  (params (Key :type Key%20Structure :default "None"))
  (bind _checkpoints (Variables|Default|GetCheckpoints))
  (bind _output (Utilities|Array|Get(acopy) _checkpoints 10))
  ;[1 1 1] Tp on checkpoint
  (:Pressed
    (if (!= _output 0)
      (if (Utilities|IsValid _output)
        (Transformation|SetActorLocation (Variables|Default|GetPlayer) (Transformation|GetActorLocation _output) false false)))))

(event Input|KeyboardEvents|Hyphen
  (params (Key :type Key%20Structure :default "None"))
  (bind _checkpoints (Variables|Default|GetCheckpoints))
  (bind _output (Utilities|Array|Get(acopy) _checkpoints 5))
  ;[1 1 1] Tp on checkpoint
  (:Pressed
    (if (!= _output 0)
      (if (Utilities|IsValid _output)
        (Transformation|SetActorLocation (Variables|Default|GetPlayer) (Transformation|GetActorLocation _output) false false)))))

(event Input|KeyboardEvents|EAccentGrave
  (params (Key :type Key%20Structure :default "None"))
  (bind _checkpoints (Variables|Default|GetCheckpoints))
  (bind _output (Utilities|Array|Get(acopy) _checkpoints 6))
  ;[1 1 1] Tp on checkpoint
  (:Pressed
    (if (!= _output 0)
      (if (Utilities|IsValid _output)
        (Transformation|SetActorLocation (Variables|Default|GetPlayer) (Transformation|GetActorLocation _output) false false)))))

(event Input|KeyboardEvents|Underscore
  (params (Key :type Key%20Structure :default "None"))
  (bind _checkpoints (Variables|Default|GetCheckpoints))
  (bind _output (Utilities|Array|Get(acopy) _checkpoints 7))
  ;[1 1 1] Tp on checkpoint
  (:Pressed
    (if (!= _output 0)
      (if (Utilities|IsValid _output)
        (Transformation|SetActorLocation (Variables|Default|GetPlayer) (Transformation|GetActorLocation _output) false false)))))

(event Input|KeyboardEvents|CCedille
  (params (Key :type Key%20Structure :default "None"))
  (bind _checkpoints (Variables|Default|GetCheckpoints))
  (bind _output (Utilities|Array|Get(acopy) _checkpoints 8))
  ;[1 1 1] Tp on checkpoint
  (:Pressed
    (if (!= _output 0)
      (if (Utilities|IsValid _output)
        (Transformation|SetActorLocation (Variables|Default|GetPlayer) (Transformation|GetActorLocation _output) false false)))))

(event Input|KeyboardEvents|AAccentGrave
  (params (Key :type Key%20Structure :default "None"))
  (bind _checkpoints (Variables|Default|GetCheckpoints))
  (bind _output (Utilities|Array|Get(acopy) _checkpoints 9))
  ;[1 1 1] Tp on checkpoint
  (:Pressed
    (if (!= _output 0)
      (if (Utilities|IsValid _output)
        (Transformation|SetActorLocation (Variables|Default|GetPlayer) (Transformation|GetActorLocation _output) false false)))))

(event Input|KeyboardEvents|Equals
  (params (Key :type Key%20Structure :default "None"))
  (bind _checkpoints (Variables|Default|GetCheckpoints))
  (bind _output (Utilities|Array|Get(acopy) _checkpoints 11))
  ;[1 1 1] Tp on checkpoint
  (:Pressed
    (if (!= _output 0)
      (if (Utilities|IsValid _output)
        (Transformation|SetActorLocation (Variables|Default|GetPlayer) (Transformation|GetActorLocation _output) false false)))))

(fn ConstructionScript)