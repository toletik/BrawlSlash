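; BP_FocusManagement shows on-screen markers for the player's current, next and previous focus targets.
; Each Tick, a shared check macro drives start, update and clear branches for each target, toggling visibility and repositioning markers.
; The main widget turns toward the camera, with timeline-driven scaling and a focus-change sound.
; Next and previous use billboards, with a combined billboard when both are the same actor.
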(event EventBeginPlay
  ;[0.5517 1 0.5386] On Begin Play: Cast Player; Set Initial Value
  (bind _ascharacter_player (Utilities|Casting|CastToCharacter_Player (Game|GetPlayerCharacter 0)))
  (Variables|Default|Setplayer _ascharacter_player)
  (Variables|MainFocus|SetmainFocus_IndicatorInitialScale (Transformation|GetWorldScale (Variables|Default|GetWDG_MainFocus_Indicator))))

(event EventTick
  (params (DeltaSeconds :type Float%20%28single-precision%29))
  (bind _returnvalue (Transformation|GetActorLocation 0))
  (bind _player (Variables|Default|Getplayer))
  (bind _billboard_nextfocus (Variables|Default|GetBillboard_NextFocus))
  (bind _player_2 (Variables|Default|Getplayer))
  (bind _player_3 (Variables|Default|Getplayer))
  (bind _player_4 (Variables|Default|GetPlayer))
  (bind _billboard_previousfocus (Variables|Default|GetBillboard_PreviousFocus))
  (bind _player_5 (Variables|Default|Getplayer))
  (bind _nextfocus_verticaloffset (Variables|NextFocus|GetnextFocus_VerticalOffset))
  (bind _player_6 (Variables|Default|GetPlayer))
  (bind _wdg_mainfocus_indicator (Variables|Default|GetWDG_MainFocus_Indicator))
  (bind _audiochangefocus (Variables|Default|GetAudioChangeFocus))
  (bind _returnvalue_2 (+ _returnvalue (Math|Vector|MakeVector 0.0 0.0 _nextfocus_verticaloffset)))
  (bind _focus (Variables|/Script/BrawlSlash.Character_Player|Getfocus _player_6))
  (bind _focus_2 (Variables|/Script/BrawlSlash.Character_Player|Getfocus _player_4))
  (bind _returnvalue_3 (Transformation|GetActorLocation _focus_2))
  (Utilities|FlowControl|Sequence
    (:then_0
      ;[1 1 1] MainFocusIndicator
      (bind _isstillthesame (Utilities|ChecksBeforeApplyingWidget _focus (Variables|MainFocus|GetcurrentMainFocus))
        (:onStart
          ;;[1 1 1] On Start Focus
          (if _isstillthesame
            (Utilities|Casting|CastToMyCharacter_EnemyBase _focus
              (:CastFailed
                (if (not (Variables|MainFocus|GetcurrentMainFocusIsTheSame))
                  (Rendering|SetVisibility (Variables|Default|GetWDG_MainFocus_Indicator) true false :!label _label)
                  (if (== (Variables|/Script/BrawlSlash.Character_Player|GetnextFocus _player) (Variables|/Script/BrawlSlash.Character_Player|GetpreviousFocus _player))
                    (Rendering|SetVisibility (Variables|Default|GetBillboard_NextFocus) false false))
                  (Audio|Components|Audio|Stop _audiochangefocus)
                  (Audio|Components|Audio|Play _audiochangefocus 0.0)
                  (Variables|MainFocus|SetcurrentMainFocusIsTheSame true)
                  (bind _focusindicator (Timeline|Timeline_0 PlayFromStart)
                    (:Update
                      (Transformation|SetWorldScale3D _wdg_mainfocus_indicator (* (Variables|MainFocus|GetmainFocus_IndicatorInitialScale) _focusindicator)))
                    (:Finished
                      _))
                  (Variables|MainFocus|SetcurrentMainFocus (Variables|/Script/BrawlSlash.Character_Player|Getfocus (Variables|Default|Getplayer))))))
            (else
              (goto _label))))
        (:Update
          ;;[1 1 1] Character Is Focussing :  Widget Position and Rotation; Color withRange
          (if (Variables|MainFocus|GetcurrentMainFocusIsTheSame)
            (if (== (Utilities|GetClass (Variables|/Script/BrawlSlash.Character_Player|Getfocus (Variables|Default|GetPlayer))) "/Game/Blueprints/LDBricks/BP_Door_Clean.BP_Door_Clean_C")
              (CallFunction|WidgetPositionandRotation _returnvalue_3 _focus_2 (Variables|Default|GetWDG_MainFocus_Indicator) (* (Variables|MainFocus|GetmainFocus_VerticalOffset) 3.0) 0.0 5e+01)
              (bind _focusindicator_2 (Timeline|Timeline_1 Play)
                (:Update
                  (Transformation|SetWorldScale3D _wdg_mainfocus_indicator (* _focusindicator_2 (Variables|MainFocus|GetmainFocus_IndicatorInitialScale)))))
              (else
                (CallFunction|WidgetPositionandRotation _returnvalue_3 _focus_2 (Variables|Default|GetWDG_MainFocus_Indicator) (Variables|MainFocus|GetmainFocus_VerticalOffset) 0.0 0.0)
                (Timeline|Timeline_1 Play)))))
        (:IfNot
          ;;[1 1 1] When no Focus Anymore
          (if (Variables|MainFocus|GetcurrentMainFocusIsTheSame)
            (Rendering|SetVisibility (Variables|Default|GetWDG_MainFocus_Indicator) false false)
            (Variables|MainFocus|SetcurrentMainFocusIsTheSame false)))))
    (:then_1
      ;[1 1 1] NextFocusIndicator
      (bind _isstillthesame_2 (Utilities|ChecksBeforeApplyingWidget (Variables|/Script/BrawlSlash.Character_Player|GetnextFocus (Variables|Default|Getplayer)) (Variables|NextFocus|GetcurrentNextFocus))
        (:onStart
          ;;[1 1 1] On Start Focus
          (if (not _isstillthesame_2)
            (if (== (Variables|/Script/BrawlSlash.Character_Player|GetnextFocus _player_3) (Variables|/Script/BrawlSlash.Character_Player|GetpreviousFocus _player_3))
              (Development|PrintString "OOOOK")
              (Rendering|SetVisibility (Variables|Default|GetBillboard_NextFocus) false false)
              (Rendering|SetVisibility (Variables|Default|GetBillboard_Next&PreviousFocus) true false)
              (else
                (Rendering|SetVisibility (Variables|Default|GetBillboard_NextFocus) true false)))
            (Variables|NextFocus|SetcurrentNextFocusIsTheSame true)
            (Variables|NextFocus|SetcurrentNextFocus (Variables|/Script/BrawlSlash.Character_Player|GetnextFocus (Variables|Default|Getplayer)))))
        (:Update
          ;;[1 1 1] Character Is Focussing :  Widget Position and Rotation;
          (if (Variables|NextFocus|GetcurrentNextFocusIsTheSame)
            (if (== (Variables|/Script/BrawlSlash.Character_Player|GetpreviousFocus _player_5) (Variables|/Script/BrawlSlash.Character_Player|GetnextFocus _player_5))
              (if (Rendering|IsVisible _billboard_nextfocus)
                (Rendering|SetVisibility _billboard_nextfocus false false))
              (Transformation|SetWorldLocation (Variables|Default|GetBillboard_Next&PreviousFocus) _returnvalue_2 false false)
              (else
                (Transformation|SetWorldLocation (Variables|Default|GetBillboard_NextFocus) _returnvalue_2 false false)))))
        (:IfNot
          ;;[1 1 1] When no Focus Anymore
          (if (Variables|NextFocus|GetcurrentNextFocusIsTheSame)
            (Rendering|SetVisibility (Variables|Default|GetBillboard_Next&PreviousFocus) false false)
            (Variables|NextFocus|SetcurrentNextFocusIsTheSame false)))))
    (:then_2
      ;[1 1 1] PreviousFocusIndicator
      (bind _isstillthesame_3 (Utilities|ChecksBeforeApplyingWidget (Variables|/Script/BrawlSlash.Character_Player|GetpreviousFocus (Variables|Default|Getplayer)) (Variables|PreviousFocus|GetcurrentPreviousFocus))
        (:onStart
          ;;[1 1 1] On Start Focus
          (if (not _isstillthesame_3)
            (if (== (Variables|/Script/BrawlSlash.Character_Player|GetpreviousFocus _player_2) (Variables|/Script/BrawlSlash.Character_Player|GetnextFocus _player_2))
              (Rendering|SetVisibility _billboard_previousfocus false false)
              (else
                (Rendering|SetVisibility _billboard_previousfocus true false)))
            (Variables|PreviousFocus|SetcurrentPreviousFocusIsTheSame true)
            (Variables|NextFocus|SetcurrentNextFocus (Variables|/Script/BrawlSlash.Character_Player|GetpreviousFocus (Variables|Default|Getplayer)))))
        (:Update
          ;;[1 1 1] Character Is Focussing :  Widget Position and Rotation;
          (if (Variables|PreviousFocus|GetcurrentPreviousFocusIsTheSame)
            (Transformation|SetWorldLocation (Variables|Default|GetBillboard_PreviousFocus) (+ (Transformation|GetActorLocation (Variables|/Script/BrawlSlash.Character_Player|GetpreviousFocus (Variables|Default|Getplayer))) (Math|Vector|MakeVector 0.0 0.0 (Variables|PreviousFocus|GetpreviousFocus_VerticalOffset))) false false)))
        (:IfNot
          ;;[1 1 1] When no Focus Anymore
          (if (Variables|PreviousFocus|GetcurrentPreviousFocusIsTheSame)
            (Rendering|SetVisibility (Variables|Default|GetBillboard_PreviousFocus) false false)
            (Variables|PreviousFocus|SetcurrentPreviousFocusIsTheSame false)))))))

(fn ConstructionScript)

(fn WidgetPositionandRotation
  (params (ActorTargetLocation :type Vector) (KindOfFocus :type Actor%20Object%20Reference) (WidgetTarget :type Scene%20Component%20Object%20Reference) (VerticalOffset :type Float%20%28single-precision%29) (LateralOffset :type Float%20%28single-precision%29) (ProfondeurOffset :type Float%20%28single-precision%29))
  (bind _returnvalue (Game|GetPlayerCameraManager 0))
  (bind _returnvalue_2 (Transformation|GetActorLocation KindOfFocus))
  (bind _returnvalue_3 (Transformation|GetActorLocation _returnvalue))
  (bind _returnvalue_4 (Math|Rotator|FindLookatRotation _returnvalue_2 _returnvalue_3))
  (Transformation|SetWorldRotation WidgetTarget (Math|Rotator|MakeRotator (.roll _returnvalue_4) (.pitch (Transformation|GetWorldRotation WidgetTarget)) (.yaw _returnvalue_4)) false false)
  (Transformation|SetWorldLocation WidgetTarget (+ ActorTargetLocation (Math|Vector|MakeVector ProfondeurOffset LateralOffset VerticalOffset)) false false))