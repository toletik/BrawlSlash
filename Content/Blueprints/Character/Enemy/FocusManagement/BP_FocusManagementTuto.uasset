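; Tutorial focus manager that shows widget indicators over the player's main, next and previous focus targets.
; Each Tick, a macro routes each target to start, update or lost logic, driving timeline scale pops, camera-facing placement and, for main focus, a sound and range-based tint.
; Dummy_AI2 gets the A indicator when facing the player, otherwise X; other targets use X.
; A combined indicator replaces next and previous when both share a target.
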(event EventBeginPlay
  ;[0.5517 1 0.5386] On Begin Play: Cast Player; Set Initial Value
  (bind _ascharacter_player (Utilities|Casting|CastToCharacter_Player (Game|GetPlayerCharacter 0)))
  (Variables|Default|Setplayer _ascharacter_player)
  (Variables|MainFocus|SetmainFocus_IndicatorInitialScale (Transformation|GetWorldScale (Variables|Default|GetWDG_MainFocus_A_Indicator)))
  (Variables|NextFocus|SetnextFocus_IndicatorInitialScale (Transformation|GetWorldScale (Variables|Default|GetWDG_NextFocus_Indicator)))
  (Variables|PreviousFocus|SetpreviousFocus_IndicatorInitialScale (Transformation|GetWorldScale (Variables|Default|GetWDG_PreviousFocus_Indicator))))

(event EventTick
  (params (DeltaSeconds :type Float%20%28single-precision%29))
  (bind _audiochangefocus (Variables|Default|GetAudioChangeFocus))
  (bind _player (Variables|Default|Getplayer))
  (bind _player_2 (Variables|Default|Getplayer))
  (bind _player_3 (Variables|Default|Getplayer))
  (bind _player_4 (Variables|Default|Getplayer))
  (bind _player_5 (Variables|Default|GetPlayer))
  (bind _player_6 (Variables|Default|GetPlayer))
  (bind _mainfocus_verticaloffset (Variables|MainFocus|GetmainFocus_VerticalOffset))
  (bind _wdg_mainfocus_x_indicator (Variables|Default|GetWDG_MainFocus_X_Indicator))
  (bind _wdg_mainfocus_x_indicator_2 (Variables|Default|GetWDG_MainFocus_X_Indicator))
  (bind _audiochangefocus_2 (Variables|Default|GetAudioChangeFocus))
  (bind _player_7 (Variables|Default|GetPlayer))
  (bind _player_8 (Variables|Default|Getplayer))
  (bind _mainfocus_verticaloffset_2 (Variables|MainFocus|GetmainFocus_VerticalOffset))
  (bind _wdg_mainfocus_a_indicator (Variables|Default|GetWDG_MainFocus_A_Indicator))
  (bind _wdg_mainfocus_x_indicator_3 (Variables|Default|GetWDG_MainFocus_X_Indicator))
  (bind _wdg_mainfocus_a_indicator_2 (Variables|Default|GetWDG_MainFocus_A_Indicator))
  (bind _wdg_mainfocus_x_indicator_4 (Variables|Default|GetWDG_MainFocus_X_Indicator))
  (bind _nextfocus_verticaloffset (Variables|NextFocus|GetnextFocus_VerticalOffset))
  (bind _player_9 (Variables|Default|GetPlayer))
  (bind _audiochangefocus_3 (Variables|Default|GetAudioChangeFocus))
  (bind _player_10 (Variables|Default|GetPlayer))
  (bind _player_11 (Variables|Default|Getplayer))
  (bind _wdg_previousfocus_indicator (Variables|Default|GetWDG_PreviousFocus_Indicator))
  (bind _previousfocus_verticaloffset (Variables|PreviousFocus|GetpreviousFocus_VerticalOffset))
  (bind _nextfocus_indicatorinitialscale (Variables|NextFocus|GetnextFocus_IndicatorInitialScale))
  (bind _returnvalue (Transformation|GetActorLocation _player_9))
  (bind _returnvalue_2 (+ "0, 0, 0" (Math|Vector|MakeVector 0.0 0.0 _mainfocus_verticaloffset_2)))
  (bind _debugnextfocus (Variables|/Script/BrawlSlash.Character_Player|GetdebugNextFocus _player))
  (bind _focus (Variables|/Script/BrawlSlash.Character_Player|Getfocus _player_9))
  (bind _focus_2 (Variables|/Script/BrawlSlash.Character_Player|Getfocus _player_6))
  (bind _focus_3 (Variables|/Script/BrawlSlash.Character_Player|Getfocus _player_5))
  (bind _focus_4 (Variables|/Script/BrawlSlash.Character_Player|Getfocus _player_7))
  (bind _focus_5 (Variables|/Script/BrawlSlash.Character_Player|Getfocus _player_10))
  (bind _debugpreviousfocus (Variables|/Script/BrawlSlash.Character_Player|GetdebugPreviousFocus _player_11))
  (bind _returnvalue_3 (Transformation|GetActorLocation _focus))
  (bind _returnvalue_4 (Transformation|GetActorForwardVector _focus))
  (bind _returnvalue_5 (Transformation|GetActorLocation _debugnextfocus))
  (bind _returnvalue_6 (- (.y _returnvalue) (.y _returnvalue_3)))
  (bind _returnvalue_7 (- (.x _returnvalue) (.x _returnvalue_3)))
  (bind _returnvalue_8 (Math|Float|Square _returnvalue_6))
  (bind _returnvalue_9 (Math|Float|Square _returnvalue_7))
  (bind _returnvalue_10 (+ _returnvalue_9 _returnvalue_8))
  (bind _returnvalue_11 (Math|Float|Sqrt _returnvalue_10))
  (bind _returnvalue_12 (/ _returnvalue_6 _returnvalue_11))
  (bind _returnvalue_13 (/ _returnvalue_7 _returnvalue_11))
  (bind _returnvalue_14 (- (.y _returnvalue_4) _returnvalue_12))
  (bind _returnvalue_15 (- (.x _returnvalue_4) _returnvalue_13))
  (bind _returnvalue_16 (Math|Float|Square _returnvalue_14))
  (bind _returnvalue_17 (Math|Float|Square _returnvalue_15))
  (bind _returnvalue_18 (+ _returnvalue_17 _returnvalue_16))
  (bind _returnvalue_19 (< _returnvalue_18 1.9))
  (Utilities|FlowControl|Sequence
    (:then_0
      (if (== (Utilities|GetClass (Variables|/Script/BrawlSlash.Character_Player|Getfocus (Variables|Default|GetPlayer))) "/Game/Blueprints/Character/Enemy/Dummy_AI2.Dummy_AI2_C")
        ;[1 1 1] Main Focus - Indicator Dummy 2
        (bind _isstillthesame (Utilities|ChecksBeforeApplyingWidget (Variables|/Script/BrawlSlash.Character_Player|Getfocus (Variables|Default|GetPlayer)) (Variables|MainFocus|GetcurrentMainFocus))
          (:onStart
            (if (not _isstillthesame)
              (if _returnvalue_19
                ;;[1 1 1] On Start Focus
                (Rendering|SetVisibility _wdg_mainfocus_x_indicator_4 false false)
                (Rendering|SetVisibility _wdg_mainfocus_a_indicator_2 true false)
                (Transformation|SetWorldLocation _wdg_mainfocus_a_indicator_2 _returnvalue_2 false false)
                (Audio|Components|Audio|Stop _audiochangefocus)
                (Audio|Components|Audio|Play _audiochangefocus 0.0)
                (Variables|MainFocus|SetcurrentMainFocusIsTheSame true)
                (bind _focusindicator (Timeline|Timeline_0 PlayFromStart)
                  (:Update
                    (Transformation|SetWorldScale3D (Variables|Default|GetWDG_MainFocus_A_Indicator) (* (Variables|MainFocus|GetmainFocus_IndicatorInitialScale) _focusindicator)))
                  (:Finished
                    _))
                (else
                  (Rendering|SetVisibility _wdg_mainfocus_a_indicator_2 false false)
                  (Rendering|SetVisibility _wdg_mainfocus_x_indicator_4 true false)
                  (Transformation|SetWorldLocation _wdg_mainfocus_x_indicator_4 _returnvalue_2 false false)
                  (Audio|Components|Audio|Stop _audiochangefocus_2)
                  (Audio|Components|Audio|Play _audiochangefocus_2 0.0)
                  (Variables|MainFocus|SetcurrentMainFocusIsTheSame true)
                  (bind _focusindicator_2 (Timeline|Timeline_6 PlayFromStart)
                    (:Update
                      (Transformation|SetWorldScale3D (Variables|Default|GetWDG_MainFocus_X_Indicator) (* (Variables|MainFocus|GetmainFocus_IndicatorInitialScale) _focusindicator_2)))
                    (:Finished
                      _))))
              (Variables|MainFocus|SetcurrentMainFocus (Variables|/Script/BrawlSlash.Character_Player|Getfocus (Variables|Default|Getplayer)) :!label _label)))
          (:Update
            (if (Variables|MainFocus|GetcurrentMainFocusIsTheSame)
              (if _returnvalue_19
                ;;[1 1 1] Character Is Focussing :  Widget Position and Rotation; Color withRange
                (Rendering|SetVisibility _wdg_mainfocus_x_indicator_2 false false)
                (Rendering|SetVisibility _wdg_mainfocus_a_indicator true false)
                (CallFunction|WidgetPositionandRotation (Transformation|GetActorLocation _focus_2) _focus_2 (Variables|Default|GetWDG_MainFocus_A_Indicator) _mainfocus_verticaloffset 0.0)
                (CallFunction|ColorwithRange (Variables|Default|GetWDG_MainFocus_A_Indicator) (Variables|MainFocus|GetmainFocus_ColorWhenShortRange) (Variables|MainFocus|GetmainFocus_ColorWhenLongRange))
                (bind _focusindicator_3 (Timeline|Timeline_7 Play)
                  (:Update
                    (Transformation|SetWorldScale3D (Variables|Default|GetWDG_MainFocus_A_Indicator) (* _focusindicator_3 (Variables|MainFocus|GetmainFocus_IndicatorInitialScale)))))
                (else
                  (Rendering|SetVisibility _wdg_mainfocus_a_indicator false false)
                  (Rendering|SetVisibility _wdg_mainfocus_x_indicator_2 true false)
                  (CallFunction|WidgetPositionandRotation (Transformation|GetActorLocation _focus_4) _focus_4 (Variables|Default|GetWDG_MainFocus_X_Indicator) _mainfocus_verticaloffset 0.0)
                  (CallFunction|ColorwithRange (Variables|Default|GetWDG_MainFocus_X_Indicator) (Variables|MainFocus|GetmainFocus_ColorWhenShortRange) (Variables|MainFocus|GetmainFocus_ColorWhenLongRange))
                  (bind _focusindicator_4 (Timeline|Timeline_4 Play)
                    (:Update
                      (Transformation|SetWorldScale3D (Variables|Default|GetWDG_MainFocus_X_Indicator) (* _focusindicator_4 (Variables|MainFocus|GetmainFocus_IndicatorInitialScale)))))))))
          (:IfNot
            ;;[1 1 1] When no Focus Anymore
            (if (Variables|MainFocus|GetcurrentMainFocusIsTheSame)
              (Rendering|SetVisibility (Variables|Default|GetWDG_MainFocus_A_Indicator) false false)
              (Variables|MainFocus|SetcurrentMainFocusIsTheSame false)
              (goto _label))))
        (else
          (bind _isstillthesame_2 (Utilities|ChecksBeforeApplyingWidget _focus_3 (Variables|MainFocus|GetcurrentMainFocus))
            (:onStart
              ;[1 1 1] MainFocus - Indicator Dummy 1
              (if _isstillthesame_2
                (Utilities|Casting|CastToMyCharacter_EnemyBase _focus_3
                  (:CastFailed
                    (if (not (Variables|MainFocus|GetcurrentMainFocusIsTheSame))
                      ;;[1 1 1] On Start Focus
                      (Rendering|SetVisibility (Variables|Default|GetWDG_MainFocus_A_Indicator) false false :!label _label_2)
                      (Rendering|SetVisibility _wdg_mainfocus_x_indicator_3 true false)
                      (Transformation|SetWorldLocation _wdg_mainfocus_x_indicator_3 (+ "0, 0, 0" (Math|Vector|MakeVector 0.0 0.0 (Variables|MainFocus|GetmainFocus_VerticalOffset))) false false)
                      (Audio|Components|Audio|Stop _audiochangefocus_3)
                      (Audio|Components|Audio|Play _audiochangefocus_3 0.0)
                      (Variables|MainFocus|SetcurrentMainFocusIsTheSame true)
                      (bind _focusindicator_5 (Timeline|Timeline_3 PlayFromStart)
                        (:Update
                          (Transformation|SetWorldScale3D (Variables|Default|GetWDG_MainFocus_X_Indicator) (* (Variables|MainFocus|GetmainFocus_IndicatorInitialScale) _focusindicator_5)))
                        (:Finished
                          _))
                      (Variables|MainFocus|SetcurrentMainFocus (Variables|/Script/BrawlSlash.Character_Player|Getfocus (Variables|Default|Getplayer)) :!label _label_3))))
                (else
                  (goto _label_2))))
            (:Update
              ;;[1 1 1] Character Is Focussing :  Widget Position and Rotation; Color withRange
              (if (Variables|MainFocus|GetcurrentMainFocusIsTheSame)
                (CallFunction|WidgetPositionandRotation (Transformation|GetActorLocation _focus_5) _focus_5 (Variables|Default|GetWDG_MainFocus_X_Indicator) (Variables|MainFocus|GetmainFocus_VerticalOffset) 0.0)
                (CallFunction|ColorwithRange _wdg_mainfocus_x_indicator (Variables|MainFocus|GetmainFocus_ColorWhenShortRange) (Variables|MainFocus|GetmainFocus_ColorWhenLongRange))
                (bind _focusindicator_6 (Timeline|Timeline_5 Play)
                  (:Update
                    (Transformation|SetWorldScale3D _wdg_mainfocus_x_indicator (* _focusindicator_6 (Variables|MainFocus|GetmainFocus_IndicatorInitialScale)))))))
            (:IfNot
              ;;[1 1 1] When no Focus Anymore
              (if (Variables|MainFocus|GetcurrentMainFocusIsTheSame)
                (Rendering|SetVisibility (Variables|Default|GetWDG_MainFocus_X_Indicator) false false)
                (Variables|MainFocus|SetcurrentMainFocusIsTheSame false)
                (goto _label_3)))))))
    (:then_1
      ;[1 1 1] NextFocusIndicator
      (bind (_isstillthesame_3 _actorlocation) (Utilities|ChecksBeforeApplyingWidget _debugnextfocus (Variables|NextFocus|GetcurrentNextFocus))
        (:onStart
          ;;[1 1 1] On Start Focus
          (if (not _isstillthesame_3)
            (if (== (Variables|/Script/BrawlSlash.Character_Player|GetdebugNextFocus _player_3) (Variables|/Script/BrawlSlash.Character_Player|GetdebugPreviousFocus _player_3))
              (Rendering|SetVisibility (Variables|Default|GetWDG_NextFocus_Indicator) false false)
              (Rendering|SetVisibility (Variables|Default|GetWDG_Next&Previous_Indicator) true false)
              (Transformation|SetWorldLocation (Variables|Default|GetWDG_Next&Previous_Indicator) (+ _actorlocation (Math|Vector|MakeVector -3e+02 0.0 _nextfocus_verticaloffset)) false false)
              (Variables|NextFocus|SetcurrentNextFocusIsTheSame true)
              (bind _focusindicator_7 (Timeline|Timeline_8 Play)
                (:Update
                  (Transformation|SetWorldScale3D (Variables|Default|GetWDG_Next&Previous_Indicator) (* _focusindicator_7 _nextfocus_indicatorinitialscale)))
                (:Finished
                  (Variables|NextFocus|SetcurrentNextFocus _debugnextfocus :!label _label_4)))
              (else
                (Rendering|SetVisibility (Variables|Default|GetWDG_NextFocus_Indicator) true false)
                (Transformation|SetWorldLocation (Variables|Default|GetWDG_NextFocus_Indicator) (+ _actorlocation (Math|Vector|MakeVector -3e+02 0.0 _nextfocus_verticaloffset)) false false)
                (Variables|NextFocus|SetcurrentNextFocusIsTheSame true)
                (bind _focusindicator_8 (Timeline|Timeline_1 PlayFromStart)
                  (:Update
                    (Transformation|SetWorldScale3D (Variables|Default|GetWDG_NextFocus_Indicator) (* _nextfocus_indicatorinitialscale _focusindicator_8)))
                  (:Finished
                    (goto _label_4)))))))
        (:Update
          ;;[1 1 1] Character Is Focussing :  Widget Position and Rotation;
          (if (Variables|NextFocus|GetcurrentNextFocusIsTheSame)
            (if (== (Variables|/Script/BrawlSlash.Character_Player|GetdebugNextFocus _player_8) (Variables|/Script/BrawlSlash.Character_Player|GetdebugPreviousFocus _player_8))
              (CallFunction|WidgetPositionandRotation _returnvalue_5 _debugnextfocus (Variables|Default|GetWDG_Next&Previous_Indicator) _nextfocus_verticaloffset 0.0)
              (else
                (CallFunction|WidgetPositionandRotation _returnvalue_5 _debugnextfocus (Variables|Default|GetWDG_NextFocus_Indicator) _nextfocus_verticaloffset 5e+01)))))
        (:IfNot
          ;;[1 1 1] When no Focus Anymore
          (if (Variables|NextFocus|GetcurrentNextFocusIsTheSame)
            (Rendering|SetVisibility (Variables|Default|GetWDG_Next&Previous_Indicator) false false)
            (Variables|NextFocus|SetcurrentNextFocusIsTheSame false)))))
    (:then_2
      ;[1 1 1] PreviousFocusIndicator
      (bind (_isstillthesame_4 _actorlocation_2) (Utilities|ChecksBeforeApplyingWidget _debugpreviousfocus (Variables|PreviousFocus|GetcurrentPreviousFocus))
        (:onStart
          ;;[1 1 1] On Start Focus
          (if (not _isstillthesame_4)
            (if (== (Variables|/Script/BrawlSlash.Character_Player|GetdebugNextFocus _player_4) (Variables|/Script/BrawlSlash.Character_Player|GetdebugPreviousFocus _player_4))
              ;;;[1 1 1] If Previous & next is the same -> Invisible
              (Rendering|SetVisibility _wdg_previousfocus_indicator false false)
              (Variables|PreviousFocus|SetcurrentPreviousFocusIsTheSame true)
              (Variables|NextFocus|SetcurrentNextFocus _debugpreviousfocus :!label _label_5)
              (else
                (Rendering|SetVisibility _wdg_previousfocus_indicator true false)
                (Transformation|SetWorldLocation _wdg_previousfocus_indicator (+ _actorlocation_2 (Math|Vector|MakeVector 0.0 0.0 _previousfocus_verticaloffset)) false false)
                (Variables|PreviousFocus|SetcurrentPreviousFocusIsTheSame true)
                (bind _focusindicator_9 (Timeline|Timeline_2 PlayFromStart)
                  (:Update
                    (Transformation|SetWorldScale3D _wdg_previousfocus_indicator (* _focusindicator_9 (Variables|PreviousFocus|GetpreviousFocus_IndicatorInitialScale))))
                  (:Finished
                    (goto _label_5)))))))
        (:Update
          ;;[1 1 1] Character Is Focussing :  Widget Position and Rotation;
          (if (Variables|PreviousFocus|GetcurrentPreviousFocusIsTheSame)
            (if (not (== (Variables|/Script/BrawlSlash.Character_Player|GetdebugNextFocus _player_2) (Variables|/Script/BrawlSlash.Character_Player|GetdebugPreviousFocus _player_2)))
              (CallFunction|WidgetPositionandRotation (Transformation|GetActorLocation _debugpreviousfocus) _debugpreviousfocus _wdg_previousfocus_indicator _previousfocus_verticaloffset -5e+01))))
        (:IfNot
          ;;[1 1 1] When no Focus Anymore
          (if (Variables|PreviousFocus|GetcurrentPreviousFocusIsTheSame)
            (Rendering|SetVisibility _wdg_previousfocus_indicator false false)
            (Variables|PreviousFocus|SetcurrentPreviousFocusIsTheSame false)))))))

(fn ConstructionScript)

(fn ColorwithRange
  (params (WidgetToColor :type Widget%20Component%20Object%20Reference) (mainFocus_ColorWhenShortRange :type Linear%20Color%20Structure) (mainFocus_ColorWhenLongRange :type Linear%20Color%20Structure))
  ;[1 1 1] Set Color with Distance
  (if (Variables|/Script/BrawlSlash.Character_Player|GetisFocusInShortRange (Variables|Default|GetPlayer))
    (if (not (Variables|MainFocus|GetmainFocus_ColoredShort))
      (Class|WidgetComponent|SetTintColorandOpacity WidgetToColor mainFocus_ColorWhenLongRange)
      (Variables|MainFocus|SetmainFocus_ColoredShort true))
    (elif (Variables|MainFocus|GetmainFocus_ColoredShort)
      (Class|WidgetComponent|SetTintColorandOpacity WidgetToColor mainFocus_ColorWhenShortRange)
      (Variables|MainFocus|SetmainFocus_ColoredShort false))))

(fn WidgetPositionandRotation
  (params (ActorTargetLocation :type Vector) (KindOfFocus :type Actor%20Object%20Reference) (WidgetTarget :type Scene%20Component%20Object%20Reference) (VerticalOffset :type Float%20%28single-precision%29) (LateralOffset :type Float%20%28single-precision%29))
  (bind _returnvalue (Transformation|GetWorldRotation WidgetTarget))
  (Transformation|SetWorldRotation WidgetTarget (Math|Rotator|MakeRotator (.roll _returnvalue) (.pitch _returnvalue) (.yaw (Math|Rotator|FindLookatRotation (Transformation|GetActorLocation KindOfFocus) (Transformation|GetActorLocation (Game|GetPlayerCameraManager 0))))) false false)
  (Transformation|SetWorldLocation WidgetTarget (+ ActorTargetLocation (Math|Vector|MakeVector 0.0 LateralOffset VerticalOffset)) false false))