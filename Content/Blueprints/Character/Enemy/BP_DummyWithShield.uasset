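; Shielded dummy enemy Blueprint that supplies audiovisual feedback for hits, shield blocks and death.
; Hit events trigger camera shake, randomized-pitch sound, blood particles, timeline-driven global time-dilation hit stop and a mesh scale punch.
; ShieldComponent front hits play particles, sound and a shield scale bounce, and the component is notified on death.
; The last death in an AI Director group adds hit stop and leaves the flash particle uncut.
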(event ShieldFrontHitted(shieldComponent)
  (bind _shieldscaleatstart (Variables|Default|GetshieldScaleAtStart))
  (bind _particlehitshieldfront (Variables|Default|GetParticleHitShieldFront))
  (Components|Activation|Activate _particlehitshieldfront true)
  (Utilities|SEHitShield)
  (Utilities|FlowControl|Delay 0.2)
  (Components|Activation|Deactivate _particlehitshieldfront)
  (bind _shieldscale (Timeline|Timeline_4 PlayFromStart)
    (:Update
      (Transformation|SetWorldScale3D (Variables|Default|GetmeshShieldFront) (* _shieldscale _shieldscaleatstart)))
    (:Finished
      (Transformation|SetWorldScale3D (Variables|Default|GetmeshShieldFront) _shieldscaleatstart))))

(event EventBeginPlay
  ;[1 1 1] Set Current Mesh Size
  (Variables|Default|SetmeshScaleAtStart (Transformation|GetWorldScale (Variables|Character|GetMesh)))
  ;[1 1 1] Get Character
  (bind _ascharacter_player (Utilities|Casting|CastToCharacter_Player (Game|GetPlayerCharacter 0)))
  (Variables|Default|SetPlayer _ascharacter_player)
  ;[1 1 1] Set Current Shield Size
  (Variables|Default|SetshieldScaleAtStart (Transformation|GetWorldScale (Variables|Default|GetmeshShieldFront)))
  ;[0.9341 1 0.9301] Set Current Shield Active
  (if (Variables|/Script/BrawlSlash.Component_EnemyShield|GetisShieldInFront (Variables|Default|GetshieldComponent))
    (Rendering|Material|SetMaterial (Variables|Default|GetmeshShieldFront) 0 "/Game/Assets/Materials/AI/M_AI_Shield/M_AI_Shield_Inst.M_AI_Shield_Inst")))

(event EventEnemyHitted
  (bind _meshscaleatstart (Variables|Default|GetmeshScaleAtStart))
  ;[1 1 1] CUSTOM EVENT: AI HasBeenHit
  (CallFunction|PlaySoundonHasBeenHit (Variables|Default|GetSE_AI_AsBeenHit))
  (Utilities|ScreenShake "/Game/Blueprints/Character/BP_Shake_AsBeenHit.BP_Shake_AsBeenHit_C")
  (bind _hitstop (Timeline|Timeline_0 PlayFromStart)
    (:Update
      (Utilities|HitStop _hitstop :!label _label)
      (Components|Activation|SetActive (Variables|Default|GetParticleBlood) true true)
      (bind _meshrescale (Timeline|Timeline_1 PlayFromStart)
        (:Update
          (Transformation|SetWorldScale3D (Variables|Character|GetMesh) (* _meshrescale _meshscaleatstart)))
        (:Finished
          (Transformation|SetWorldScale3D (Variables|Character|GetMesh) _meshscaleatstart))))
    (:Finished
      (goto _label Finished))))

(event EventLastEnemyinGroup
  ;[1 1 1] On Last AI Death of AIDirector
  (Utilities|ScreenShake "/Game/Blueprints/Character/BP_Shake_AI_LastDeath.BP_Shake_AI_LastDeath_C")
  (Class|ComponentEnemyShield|OnOwnerDeath (Variables|Default|GetshieldComponent))
  (Utilities|ParticleFlashEffect 0.6 false (Variables|Default|GetParticleFlash))
  (bind _hitstop (Timeline|Timeline_2 PlayFromStart)
    (:Update
      (Utilities|HitStop _hitstop :!label _label))
    (:Finished
      (goto _label Finished))))

(event EventEnemyDeath
  ;[1 1 1] Dummy Death
  (Utilities|ScreenShake "/Game/Blueprints/Character/BP_Shake_AI_LastDeath.BP_Shake_AI_LastDeath_C")
  (Class|ComponentEnemyShield|OnOwnerDeath (Variables|Default|GetshieldComponent))
  (Utilities|ParticleFlashEffect 0.1 true (Variables|Default|GetParticleFlash))
  (Audio|PlaySound2D "/Game/Assets/Sounds/LDBricks/SE_WoodHit.SE_WoodHit" 1.0 1.0 0.0 0 0)
  (Components|Activation|SetActive (Variables|Default|GetParticleBlood) true true))

(fn ConstructionScript)

(fn PlaySoundonHasBeenHit
  (params (SE_HasBeenHit :type Audio%20Component%20Object%20Reference))
  (Audio|Components|Audio|SetPitchMultiplier SE_HasBeenHit (Math|Random|RandomFloatinRange 0.8 1.0))
  (Audio|Components|Audio|Stop SE_HasBeenHit)
  (Audio|Components|Audio|Play SE_HasBeenHit 0.0)
  (return))