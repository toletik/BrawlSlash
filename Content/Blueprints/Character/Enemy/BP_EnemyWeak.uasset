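; Weak enemy character Blueprint that handles visual, audio and game-feel feedback for combat states.
; AnimBp_EnemyWeak dispatchers for attack startup, active and recovery drive the decal indicator, sword trails and timeline-based weapon scale pulses.
; Fight-start, need-attack, hit and death events trigger indicators, camera shakes, and on hit, sound, blood and mesh rescaling.
; Hits and the group's last death add hit stop via timeline-driven global time dilation.
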(event Custom|AI1-2_EndAttack
  ;[1 1 1] On AI 1-2 WA
  (Rendering|SetVisibility (Variables|Default|GetAttackStateIndicator) false false)
  (Components|Activation|Deactivate (Variables|Default|GetP_TA_Trails_1))
  (Components|Activation|Deactivate (Variables|Default|GetP_TA_Trails_2)))

(event Custom|Attack_Startup_Event_1
  ;[1 1 1] On AI 1-2 WA
  (Rendering|SetVisibility (Variables|Default|GetAttackStateIndicator) true false)
  (Rendering|Components|Decal|SetDecalMaterial (Variables|Default|GetAttackStateIndicator) "/Game/Assets/Materials/AI/M_AI_IsAttacking/M_AI_IsAttacking_Inst2.M_AI_IsAttacking_Inst2")
  (Components|Activation|Activate (Variables|Default|GetP_TA_Trails_1) true)
  (Components|Activation|Activate (Variables|Default|GetP_TA_Trails_2) true))

(event Custom|Attack_Active_Event_0
  (bind _weaponscaleatstart (Variables|Default|GetweaponScaleAtStart))
  ;[1 1 1] On AI 1-2 WA
  (Rendering|Components|Decal|SetDecalMaterial (Variables|Default|GetAttackStateIndicator) "/Game/Assets/Materials/AI/M_AI_IsAttacking/M_AI_IsAttacking_Inst3.M_AI_IsAttacking_Inst3")
  (Utilities|FlowControl|Sequence
    (:then_0
      (bind _focusindicator_rescale (Timeline|Timeline_4 PlayFromStart)
        (:Update
          (Transformation|SetWorldScale3D (Variables|Default|GetAttackStateIndicator) (* _focusindicator_rescale (Variables|Default|GetattackStateIndicatorScale))))))
    (:then_1
      (bind _wa_weaponrescale (Timeline|Timeline_5 PlayFromStart)
        (:Update
          (Transformation|SetWorldScale3D (Variables|Default|GetSword02SM_1) (* _wa_weaponrescale _weaponscaleatstart))
          (Transformation|SetWorldScale3D (Variables|Default|GetSword02SM_2) (* _wa_weaponrescale _weaponscaleatstart)))
        (:Finished
          (Transformation|SetWorldScale3D (Variables|Default|GetSword02SM_1) _weaponscaleatstart))))))

(event Custom|EnemyStartNeedAttackWeak_1
  (bind _attackstateindicator (Variables|Default|GetAttackStateIndicator))
  ;[1 1 1] When Need To Attack (Weak Attack) : Attack Sign
  (Rendering|SetVisibility _attackstateindicator true false)
  (Rendering|Components|Decal|SetDecalMaterial _attackstateindicator "/Game/Assets/Materials/AI/M_AI_IsAttacking/M_AI_IsAttacking_Inst2.M_AI_IsAttacking_Inst2"))

(event EventBeginPlay
  ;[1 1 1] Set Current Weapon Size
  (Variables|Default|SetweaponScaleAtStart (Transformation|GetWorldScale (Variables|Default|GetSword02SM_1)))
  ;[1 1 1] Set Current Mesh Size
  (Variables|Default|SetmeshScaleAtStart (Transformation|GetWorldScale (Variables|Character|GetMesh)))
  ;[1 1 1] Get Character
  (bind _ascharacter_player (Utilities|Casting|CastToCharacter_Player (Game|GetPlayerCharacter 0)))
  (Variables|Default|SetPlayer _ascharacter_player)
  ;[1 1 1] Get Indicators Scales
  (Variables|Default|SetattackStateIndicatorScale (Transformation|GetWorldScale (Variables|Default|GetAttackStateIndicator)))
  (Variables|Default|SetfightIndicatorScale (Transformation|GetWorldScale (Variables|Default|GetFightIndicator)))
  ;[1 1 1] On AI 1-2 WA
  (bind _asanim_bp_enemy_weak (Utilities|Casting|CastToAnimBp_EnemyWeak (Components|SkeletalMesh|GetAnimInstance (Variables|Character|GetMesh))))
  (EventDispatchers|AssignWAStartup _asanim_bp_enemy_weak (delegate Custom|Attack_Startup_Event_1))
  (EventDispatchers|AssignWAActive _asanim_bp_enemy_weak (delegate Custom|Attack_Active_Event_0))
  (EventDispatchers|AssignWARecovery _asanim_bp_enemy_weak (delegate Custom|AI1-2_EndAttack)))

(event EventEnemyDeath
  ;[1 1 1] Enemy Weak Death
  (Utilities|ScreenShake "/Game/Blueprints/Character/BP_Shake_AI_Death.BP_Shake_AI_Death_C")
  (Rendering|SetVisibility (Variables|Default|GetAttackStateIndicator) false false)
  (Components|Activation|Deactivate (Variables|Default|GetP_TA_Trails_1))
  (Components|Activation|Deactivate (Variables|Default|GetP_TA_Trails_2)))

(event EventEnemyHitted
  (bind _meshscaleatstart (Variables|Default|GetmeshScaleAtStart))
  ;[1 1 1] CUSTOM EVENT: AI HasBeenHit
  (CallFunction|PlaySoundonHasBeenHit (Variables|Default|GetSE_AI_AsBeenHit))
  (Utilities|ScreenShake "/Game/Blueprints/Character/BP_Shake_AsBeenHit.BP_Shake_AsBeenHit_C")
  (bind _hitstop (Timeline|Timeline_0 PlayFromStart)
    (:Update
      (Utilities|HitStop _hitstop :!label _label)
      (Components|Activation|SetActive (Variables|Default|GetParticleBlood) true true)
      (bind _meshrescale (Timeline|Timeline_1 PlayFromStart)
        (:Update
          (Transformation|SetWorldScale3D (Variables|Character|GetMesh) (* _meshrescale _meshscaleatstart)))
        (:Finished
          (Transformation|SetWorldScale3D (Variables|Character|GetMesh) _meshscaleatstart))))
    (:Finished
      (goto _label Finished))))

(event EventLastEnemyinGroup
  ;[1 1 1] On Last AI Death of AIDirector
  (Utilities|ScreenShake "/Game/Blueprints/Character/BP_Shake_AI_LastDeath.BP_Shake_AI_LastDeath_C")
  (Rendering|SetVisibility (Variables|Default|GetAttackStateIndicator) false false)
  (Components|Activation|Deactivate (Variables|Default|GetP_TA_Trails_1))
  (Utilities|ParticleFlashEffect 0.6 true (Variables|Default|GetParticleFlash))
  (bind _hitstop (Timeline|Timeline_2 PlayFromStart)
    (:Update
      (Utilities|HitStop _hitstop :!label _label))
    (:Finished
      (goto _label Finished))))

(event EventEnemyStartFight
  (bind _returnvalue (Transformation|GetActorLocation))
  (bind _fightindicator (Variables|Default|GetFightIndicator))
  ;[1 1 1] Fight Indicator : Surpise Sign
  (Rendering|SetVisibility _fightindicator true false)
  (Transformation|SetWorldLocation _fightindicator (Math|Vector|MakeVector (.x _returnvalue) (.y _returnvalue) (+ (.z _returnvalue) 3e+02)) false false)
  (bind _opacityovertime (Timeline|Timeline_3 PlayFromStart)
    (:Update
      (Transformation|SetWorldScale3D _fightindicator (Math|Vector|MakeVector (+ _opacityovertime 1.0) (+ _opacityovertime 1.0) (+ _opacityovertime 1.0)))
      (Class|WidgetComponent|SetTintColorandOpacity _fightindicator (Utilities|Struct|MakeLinearColor 1.0 0.166518 0.0 _opacityovertime))
      (CallFunction|WDGFightIndicatorRotation (Variables|Default|GetFightIndicator)))
    (:Finished
      (Rendering|SetVisibility _fightindicator false false))))

(fn ConstructionScript)

(fn PlaySoundonHasBeenHit
  (params (SE_HasBeenHit :type Audio%20Component%20Object%20Reference))
  (Audio|Components|Audio|SetPitchMultiplier SE_HasBeenHit (Math|Random|RandomFloatinRange 0.8 1.0))
  (Audio|Components|Audio|Stop SE_HasBeenHit)
  (Audio|Components|Audio|Play SE_HasBeenHit 0.0)
  (return))

(fn WDGFightIndicatorRotation
  (params (FightIndicator :type Scene%20Component%20Object%20Reference))
  (bind _returnvalue (Game|GetPlayerCameraManager 0))
  (bind _returnvalue_2 (Transformation|GetActorLocation))
  (bind _returnvalue_3 (Transformation|GetActorLocation _returnvalue))
  (bind _returnvalue_4 (Math|Rotator|FindLookatRotation _returnvalue_2 _returnvalue_3))
  (Transformation|SetWorldRotation FightIndicator (Math|Rotator|MakeRotator (.roll _returnvalue_4) (.pitch (Transformation|GetWorldRotation FightIndicator)) (.yaw _returnvalue_4)) false false)
  (return))