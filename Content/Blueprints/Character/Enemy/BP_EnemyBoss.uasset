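; Boss enemy Blueprint that drives the audiovisual and gamepad feedback for its attacks, shields, hits and death.
; AnimBp_EnemyBoss dispatchers time the cone (SA) and randomly rotated circle (RA) attack telegraphs, decals, particles and rumble.
; ShieldComponent events swap front/back shield materials and trigger impact effects, while timelines pulse mesh, weapon and indicator scales.
; Hits and last-in-group death add global time-dilation hit stop; both death events play staggered flash-and-sound bursts.
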(event EnemyShieldFrontStartActive(shieldComponent)
  ;[1 1 1] Shield : Activations , Deactivations
  (Rendering|Material|SetMaterial (Variables|Default|GetmeshShieldFront) 0 "/Game/Assets/Materials/AI/M_AI_Shield/M_AI_Shield_Inst.M_AI_Shield_Inst"))

(event EnemyShieldFrontStarttoActive(shieldComponent)
  ;[1 1 1] Shield : Activations , Deactivations
  (Rendering|Material|SetMaterial (Variables|Default|GetmeshShieldFront) 0 "/Game/Assets/Materials/AI/M_AI_Shield/M_AI_Shield_Inst_2.M_AI_Shield_Inst_2"))

(event EnemyShieldFrontStarttoDeactive(shieldComponent)
  ;[1 1 1] Shield : Activations , Deactivations
  (Rendering|Material|SetMaterial (Variables|Default|GetmeshShieldFront) 0 "/Game/Assets/Materials/AI/M_AI_Shield/M_AI_Shield_Inst_3.M_AI_Shield_Inst_3"))

(event EnemyShieldBackStartActive(shieldComponent)
  ;[1 1 1] Shield : Activations , Deactivations
  (Rendering|Material|SetMaterial (Variables|Default|GetmeshShieldBack) 0 "/Game/Assets/Materials/AI/M_AI_Shield/M_AI_Shield_Inst.M_AI_Shield_Inst"))

(event EnemyShieldBackStarttoActive(shieldComponent)
  ;[1 1 1] Shield : Activations , Deactivations
  (Rendering|Material|SetMaterial (Variables|Default|GetmeshShieldBack) 0 "/Game/Assets/Materials/AI/M_AI_Shield/M_AI_Shield_Inst_2.M_AI_Shield_Inst_2"))

(event EnemyShieldBackStarttoDeactive(shieldComponent)
  ;[1 1 1] Shield : Activations , Deactivations
  (Rendering|Material|SetMaterial (Variables|Default|GetmeshShieldBack) 0 "/Game/Assets/Materials/AI/M_AI_Shield/M_AI_Shield_Inst_3.M_AI_Shield_Inst_3"))

(event ShieldBackHitted(shieldComponent)
  (bind _shieldscaleatstart (Variables|Default|GetshieldScaleAtStart))
  (bind _particlehitshieldback (Variables|Default|GetParticleHitShieldBack))
  ;[1 1 1] On Hit Shield
  (Utilities|ScreenShake "/Game/Blueprints/Character/BP_Shake_AsBeenHit.BP_Shake_AsBeenHit_C")
  (Components|Activation|Activate _particlehitshieldback true)
  (Utilities|SEHitShield)
  (Utilities|FlowControl|Delay 0.2)
  (Components|Activation|Deactivate _particlehitshieldback)
  (bind _shieldscale (Timeline|Timeline_6 PlayFromStart)
    (:Update
      (Transformation|SetWorldScale3D (Variables|Default|GetmeshShieldBack) (* _shieldscale _shieldscaleatstart)))
    (:Finished
      (Transformation|SetWorldScale3D (Variables|Default|GetmeshShieldBack) _shieldscaleatstart))))

(event ShieldFrontHitted(shieldComponent)
  (bind _shieldscaleatstart (Variables|Default|GetshieldScaleAtStart))
  (bind _particlehitshieldfront (Variables|Default|GetParticleHitShieldFront))
  ;[1 1 1] On Hit Shield
  (Utilities|ScreenShake "/Game/Blueprints/Character/BP_Shake_AsBeenHit.BP_Shake_AsBeenHit_C")
  (Components|Activation|Activate _particlehitshieldfront true)
  (Utilities|SEHitShield)
  (Utilities|FlowControl|Delay 0.2)
  (Components|Activation|Deactivate _particlehitshieldfront)
  (bind _shieldscale (Timeline|Timeline_7 PlayFromStart)
    (:Update
      (Transformation|SetWorldScale3D (Variables|Default|GetmeshShieldFront) (* _shieldscale _shieldscaleatstart)))
    (:Finished
      (Transformation|SetWorldScale3D (Variables|Default|GetmeshShieldFront) _shieldscaleatstart))))

(event Custom|AI4_ConeAttack_Startup
  ;[1 1 1] On AI 4 SA & RA
  (CallFunction|ConeAttackSAStartUp))

(event Custom|AI4_SA_Active
  (bind _weaponscaleatstart (Variables|Default|GetweaponScaleAtStart))
  ;[1 1 1] On AI 4 SA & RA
  (Rendering|SetVisibility (Variables|Default|GetSM_AI_SA_StartUp) false false)
  (Components|Activation|Activate (Variables|Default|GetP_AI_SA_Active) true)
  (Components|Activation|Deactivate (Variables|Default|GetP_TA_Trails_1))
  (Rendering|Components|Decal|SetDecalMaterial (Variables|Default|GetAttackStateIndicator) "/Game/Assets/Materials/AI/M_AI_IsAttacking/M_AI_IsAttacking_Inst3.M_AI_IsAttacking_Inst3")
  (Game|Feedback|ClientPlayForceFeedback (Game|GetPlayerController 0) "/Game/Assets/ControllerFeedback/FE_AI4_Attack.FE_AI4_Attack" "None" true false false)
  (Utilities|FlowControl|Sequence
    (:then_0
      (bind _sa_weaponrescale (Timeline|Timeline_5 PlayFromStart)
        (:Update
          (Transformation|SetWorldScale3D (Variables|Default|GetSword02SM_1) (* _sa_weaponrescale _weaponscaleatstart)))
        (:Finished
          (Transformation|SetWorldScale3D (Variables|Default|GetSword02SM_1) _weaponscaleatstart))))
    (:then_1
      (bind _focusindicator_rescale (Timeline|Timeline_4 PlayFromStart)
        (:Update
          (Transformation|SetWorldScale3D (Variables|Default|GetAttackStateIndicator) (* _focusindicator_rescale (Variables|Default|GetattackStateIndicatorScale))))))))

(event Custom|AI4_RA_Active
  (bind _attackcircleangle (Variables|Default|GetattackCircleAngle))
  (bind _weaponscaleatstart (Variables|Default|GetweaponScaleAtStart))
  ;[1 1 1] On AI 4 SA & RA
  (Transformation|SetRelativeRotation (Variables|Default|GetattackMeshCircle) (Math|Rotator|MakeRotator 0.0 0.0 _attackcircleangle) false false)
  (Transformation|SetRelativeRotation (Variables|Default|GetP_AI4_RA_Active) (Math|Rotator|MakeRotator 0.0 0.0 _attackcircleangle) false false)
  (Components|Activation|Activate (Variables|Default|GetP_AI4_RA_Active) true)
  (Components|Activation|Deactivate (Variables|Default|GetP_TA_Trails_1))
  (Rendering|Components|Decal|SetDecalMaterial (Variables|Default|GetAttackStateIndicator) "/Game/Assets/Materials/AI/M_AI_IsAttacking/M_AI_IsAttacking_Inst3.M_AI_IsAttacking_Inst3")
  (Game|Feedback|ClientPlayForceFeedback (Game|GetPlayerController 0) "/Game/Assets/ControllerFeedback/FE_AI4_Attack.FE_AI4_Attack" "None" true false false)
  (Utilities|FlowControl|Sequence
    (:then_0
      (bind _sa_weaponrescale (Timeline|Timeline_5 PlayFromStart)
        (:Update
          (Transformation|SetWorldScale3D (Variables|Default|GetSword02SM_1) (* _sa_weaponrescale _weaponscaleatstart)))
        (:Finished
          (Transformation|SetWorldScale3D (Variables|Default|GetSword02SM_1) _weaponscaleatstart))))
    (:then_1
      (bind _focusindicator_rescale (Timeline|Timeline_4 PlayFromStart)
        (:Update
          (Transformation|SetWorldScale3D (Variables|Default|GetAttackStateIndicator) (* _focusindicator_rescale (Variables|Default|GetattackStateIndicatorScale))))))))

(event Custom|AI4_RA_Startup
  ;[1 1 1] On AI 4 SA & RA
  (Rendering|SetVisibility (Variables|Default|GetAttackStateIndicator) true false)
  (Components|Activation|Activate (Variables|Default|GetP_AI4_RA_Startup) true)
  (Rendering|Components|Decal|SetDecalMaterial (Variables|Default|GetAttackStateIndicator) "/Game/Assets/Materials/AI/M_AI_IsAttacking/M_AI_IsAttacking_Inst2.M_AI_IsAttacking_Inst2")
  (Variables|Default|SetattackCircleAngle (Math|Random|RandomFloatinRange -1.8e+02 1.8e+02))
  (Transformation|SetRelativeRotation (Variables|Default|GetP_AI4_RA_Startup) (Math|Rotator|MakeRotator 0.0 0.0 (Variables|Default|GetattackCircleAngle)) false false)
  (Components|Activation|Activate (Variables|Default|GetP_TA_Trails_1) true))

(event Custom|AI4_EndAttack
  ;[1 1 1] On AI 4 SA & RA
  (Rendering|SetVisibility (Variables|Default|GetAttackStateIndicator) false false)
  (Game|Feedback|ClientStopForceFeedback (Game|GetPlayerController 0) "/Game/Assets/ControllerFeedback/FE_AI4_Attack.FE_AI4_Attack" "None"))

(event EventBeginPlay
  (bind _shieldcomponent (Variables|Default|GetshieldComponent))
  ;[1 1 1] Set Current Shield Size
  (Variables|Default|SetshieldScaleAtStart (Transformation|GetWorldScale (Variables|Default|GetmeshShieldFront)))
  ;[1 1 1] Set Current Weapon Size
  (Variables|Default|SetweaponScaleAtStart (Transformation|GetWorldScale (Variables|Default|GetSword02SM_1)))
  ;[1 1 1] Set Current Mesh Size
  (Variables|Default|SetmeshScaleAtStart (Transformation|GetWorldScale (Variables|Character|GetMesh)))
  ;[1 1 1] Get Character
  (bind _ascharacter_player (Utilities|Casting|CastToCharacter_Player (Game|GetPlayerCharacter 0)))
  (Variables|Default|SetPlayer _ascharacter_player)
  ;[1 1 1] Get Indicators Scales
  (Variables|Default|SetattackStateIndicatorScale (Transformation|GetWorldScale (Variables|Default|GetAttackStateIndicator)))
  (Variables|Default|SetfightIndicatorScale (Transformation|GetWorldScale (Variables|Default|GetFightIndicator)))
  ;[0.9341 1 0.9301] Set Current Shield Active
  (if (Variables|/Script/BrawlSlash.Component_EnemyShield|GetisShieldInFront _shieldcomponent)
    (Rendering|Material|SetMaterial (Variables|Default|GetmeshShieldFront) 0 "/Game/Assets/Materials/AI/M_AI_Shield/M_AI_Shield_Inst.M_AI_Shield_Inst"))
  (if (Variables|/Script/BrawlSlash.Component_EnemyShield|GetisShieldInBack _shieldcomponent)
    (Rendering|Material|SetMaterial (Variables|Default|GetmeshShieldBack) 0 "/Game/Assets/Materials/AI/M_AI_Shield/M_AI_Shield_Inst.M_AI_Shield_Inst"))
  ;[1 1 1] Health Bar
  (bind _aswdg_hud_ai4 (Utilities|Casting|CastToWDG_HUD_AI4 (UserInterface|GetUserWidgetObject (Variables|Default|GetHealthBar))))
  (Variables|/Game/Blueprints/UI/WDG_HUD_AI4.WDG_HUD_AI4_C|SetenemyRef _aswdg_hud_ai4 self)
  ;[1 1 1] On AI 4 SA & RA
  (bind _asanim_bp_enemy_boss (Utilities|Casting|CastToAnimBp_EnemyBoss (Components|SkeletalMesh|GetAnimInstance (Variables|Character|GetMesh))))
  (EventDispatchers|AssignAI4SAStartup _asanim_bp_enemy_boss (delegate Custom|AI4_ConeAttack_Startup))
  (EventDispatchers|AssignAI4RAStartup _asanim_bp_enemy_boss (delegate Custom|AI4_RA_Startup))
  (EventDispatchers|AssignAI4SAActive _asanim_bp_enemy_boss (delegate Custom|AI4_SA_Active))
  (EventDispatchers|AssignAI4RAActive _asanim_bp_enemy_boss (delegate Custom|AI4_RA_Active))
  (EventDispatchers|BindEventtoAI4SARecovery _asanim_bp_enemy_boss (delegate Custom|AI4_EndAttack))
  (EventDispatchers|AssignAI4RAEnd _asanim_bp_enemy_boss (delegate Custom|AI4_EndAttack)))

(event EventEnemyDeath
  (bind _self self)
  (bind _returnvalue (Transformation|GetActorLocation _self))
  (bind _returnvalue_2 (+ (.x _returnvalue) 3e+02))
  (bind _returnvalue_3 (+ (.y _returnvalue) -2e+02))
  (bind _returnvalue_4 (+ (.z _returnvalue) 5e+01))
  ;[1 1 1] Boss Death
  (Utilities|ScreenShake "/Game/Blueprints/Character/BP_Shake_AI_LastDeath.BP_Shake_AI_LastDeath_C")
  (Rendering|SetVisibility (Variables|Default|GetAttackStateIndicator) false false)
  (Components|Activation|Deactivate (Variables|Default|GetP_TA_Trails_1))
  (Class|ComponentEnemyShield|OnOwnerDeath (Variables|Default|GetshieldComponent))
  (Rendering|SetVisibility (Variables|Default|GetSM_AI_SA_StartUp) false false)
  (Game|Feedback|ClientStopForceFeedback (Game|GetPlayerController 0) "/Game/Assets/ControllerFeedback/FE_AI4_Attack.FE_AI4_Attack" "None")
  (bind _returnvalue_5 (Effects|SpawnEmitteratLocation "/Game/Assets/VisualEffects/AI/P_AI_Death_Flash.P_AI_Death_Flash" (Math|Vector|MakeVector (+ (.x _returnvalue) 2e+02) (+ (.y _returnvalue) 2e+02) (+ (.z _returnvalue) -5e+01)) "75.000000, 0,60.000000" "1.500000,1.000000,1.000000"))
  (Audio|PlaySoundatLocation "/Game/Assets/Sounds/LDBricks/SE_LD_BridgeOpening.SE_LD_BridgeOpening" (Math|Vector|MakeVector (.x _returnvalue) (.y _returnvalue) (.z _returnvalue)) "0, 0, 0" 0.7 1.0 0.0 0 0 0)
  (Utilities|FlowControl|Delay 0.3)
  (bind _returnvalue_6 (Effects|SpawnEmitteratLocation "/Game/Assets/VisualEffects/AI/P_AI_Death_Flash.P_AI_Death_Flash" (Math|Vector|MakeVector (+ (.x _returnvalue) -3e+02) (+ (.y _returnvalue) -3e+02) (+ (.z _returnvalue) 1e+02))))
  (Audio|PlaySoundatLocation "/Game/Assets/Sounds/LDBricks/SE_LD_BridgeOpening.SE_LD_BridgeOpening" (Math|Vector|MakeVector (.x _returnvalue) (.y _returnvalue) 0.0) "0, 0, 0" 0.7 1.0 0.0 0 0 0)
  (Utilities|FlowControl|Delay 0.4)
  (bind _returnvalue_7 (Effects|SpawnEmitteratLocation "/Game/Assets/VisualEffects/AI/P_AI_Death_Flash.P_AI_Death_Flash" (Math|Vector|MakeVector _returnvalue_2 _returnvalue_3 _returnvalue_4) "90.000000, 0, 0" "0.800000,0.600000,1.200000"))
  (Audio|PlaySoundatLocation "/Game/Assets/Sounds/LDBricks/SE_LD_BridgeOpening.SE_LD_BridgeOpening" (Math|Vector|MakeVector _returnvalue_2 _returnvalue_3 _returnvalue_4) "0, 0, 0" 0.7 1.0 0.0 0 0 0)
  (Utilities|FlowControl|Delay 0.5)
  (Components|DestroyComponent _returnvalue_5)
  (Components|DestroyComponent (Variables|Default|GetattackMeshCircle))
  (Components|DestroyComponent (Variables|Default|GetattackMeshStrong)))

(event EventEnemyHitted
  (bind _meshscaleatstart (Variables|Default|GetmeshScaleAtStart))
  ;[1 1 1] CUSTOM EVENT: AI HasBeenHit
  (CallFunction|PlaySoundonHasBeenHit (Variables|Default|GetSE_AI_AsBeenHit) 0.6 0.7)
  (Utilities|ScreenShake "/Game/Blueprints/Character/BP_Shake_AsBeenHit.BP_Shake_AsBeenHit_C")
  (bind _hitstop (Timeline|Timeline_0 PlayFromStart)
    (:Update
      (Utilities|HitStop _hitstop :!label _label)
      (Components|Activation|SetActive (Variables|Default|GetParticleBlood) true true)
      (bind _meshrescale (Timeline|Timeline_1 PlayFromStart)
        (:Update
          (Transformation|SetWorldScale3D (Variables|Character|GetMesh) (* _meshrescale _meshscaleatstart)))
        (:Finished
          (Transformation|SetWorldScale3D (Variables|Character|GetMesh) _meshscaleatstart))))
    (:Finished
      (goto _label Finished))))

(event EventLastEnemyinGroup
  (bind _self self)
  (bind _returnvalue (Transformation|GetActorLocation _self))
  (bind _returnvalue_2 (+ (.z _returnvalue) -1.5e+02))
  (bind _returnvalue_3 (+ (.x _returnvalue) 3e+02))
  (bind _returnvalue_4 (+ (.y _returnvalue) -2e+02))
  ;[1 1 1] On Last AI Death of AIDirector
  (Utilities|ScreenShake "/Game/Blueprints/Character/BP_Shake_AI_LastDeath.BP_Shake_AI_LastDeath_C")
  (Rendering|SetVisibility (Variables|Default|GetAttackStateIndicator) false false)
  (Rendering|SetVisibility (Variables|Default|GetSM_AI_SA_StartUp) false false)
  (Components|Activation|Deactivate (Variables|Default|GetP_TA_Trails_1))
  (Class|ComponentEnemyShield|OnOwnerDeath (Variables|Default|GetshieldComponent))
  (Game|Feedback|ClientStopForceFeedback (Game|GetPlayerController 0) "/Game/Assets/ControllerFeedback/FE_AI4_Attack.FE_AI4_Attack" "None")
  (Utilities|FlowControl|Sequence
    (:then_0
      (bind _hitstop (Timeline|Timeline_2 PlayFromStart)
        (:Update
          (Utilities|HitStop _hitstop :!label _label))
        (:Finished
          (goto _label Finished))))
    (:then_1
      (bind _returnvalue_5 (Effects|SpawnEmitteratLocation "/Game/Assets/VisualEffects/AI/P_AI_Death_Flash.P_AI_Death_Flash" (Math|Vector|MakeVector (+ (.x _returnvalue) 2e+02) (+ (.y _returnvalue) 2e+02) (+ (.z _returnvalue) -1e+02)) "75.000000, 0,60.000000" "1.500000,1.000000,1.000000"))
      (Audio|PlaySoundatLocation "/Game/Assets/Sounds/LDBricks/SE_LD_BridgeOpening.SE_LD_BridgeOpening" (Math|Vector|MakeVector (.x _returnvalue) (.y _returnvalue) (.z _returnvalue)) "0, 0, 0" 0.7 1.0 0.0 0 0 0)
      (Utilities|FlowControl|Delay 0.3)
      (bind _returnvalue_6 (Effects|SpawnEmitteratLocation "/Game/Assets/VisualEffects/AI/P_AI_Death_Flash.P_AI_Death_Flash" (Math|Vector|MakeVector (+ (.x _returnvalue) -3e+02) (+ (.y _returnvalue) -3e+02) (+ (.z _returnvalue) -5e+01))))
      (Audio|PlaySoundatLocation "/Game/Assets/Sounds/LDBricks/SE_LD_BridgeOpening.SE_LD_BridgeOpening" (Math|Vector|MakeVector (.x _returnvalue) (.y _returnvalue) 0.0) "0, 0, 0" 0.7 1.0 0.0 0 0 0)
      (Utilities|FlowControl|Delay 0.4)
      (bind _returnvalue_7 (Effects|SpawnEmitteratLocation "/Game/Assets/VisualEffects/AI/P_AI_Death_Flash.P_AI_Death_Flash" (Math|Vector|MakeVector _returnvalue_3 _returnvalue_4 _returnvalue_2) "90.000000, 0, 0" "0.800000,0.600000,1.200000"))
      (Audio|PlaySoundatLocation "/Game/Assets/Sounds/LDBricks/SE_LD_BridgeOpening.SE_LD_BridgeOpening" (Math|Vector|MakeVector _returnvalue_3 _returnvalue_4 _returnvalue_2) "0, 0, 0" 0.7 1.0 0.0 0 0 0)
      (Utilities|FlowControl|Delay 0.5)
      (Components|DestroyComponent _returnvalue_5)
      (Components|DestroyComponent (Variables|Default|GetattackMeshCircle))
      (Components|DestroyComponent (Variables|Default|GetattackMeshStrong)))))

(event EventEnemyStartFight
  (bind _fightindicator (Variables|Default|GetFightIndicator))
  ;[1 1 1] Fight Indicator : Surpise Sign
  (Rendering|SetVisibility _fightindicator true false)
  (bind _opacityovertime (Timeline|Timeline_3 PlayFromStart)
    (:Update
      (Transformation|SetWorldScale3D _fightindicator (Math|Vector|MakeVector (+ _opacityovertime 1.0) (+ _opacityovertime 1.0) (+ _opacityovertime 1.0)))
      (Class|WidgetComponent|SetTintColorandOpacity _fightindicator (Utilities|Struct|MakeLinearColor 1.0 0.166518 0.0 _opacityovertime)))
    (:Finished
      (Rendering|SetVisibility (Variables|Default|GetFightIndicator) false false))))

(fn ConstructionScript)

(fn PlaySoundonHasBeenHit
  (params (SE_HasBeenHit :type Audio%20Component%20Object%20Reference) (Min :type Float%20%28single-precision%29) (Max :type Float%20%28single-precision%29))
  (Audio|Components|Audio|SetPitchMultiplier SE_HasBeenHit (Math|Random|RandomFloatinRange Min Max))
  (Audio|Components|Audio|Stop SE_HasBeenHit)
  (Audio|Components|Audio|Play SE_HasBeenHit 0.0)
  (return))

(fn WDGFightIndicatorRotation
  (params (FightIndicator :type Scene%20Component%20Object%20Reference))
  (bind _returnvalue (Game|GetPlayerCameraManager 0))
  (bind _returnvalue_2 (Transformation|GetActorLocation))
  (bind _returnvalue_3 (Transformation|GetActorLocation _returnvalue))
  (bind _returnvalue_4 (Math|Rotator|FindLookatRotation _returnvalue_2 _returnvalue_3))
  (Transformation|SetWorldRotation FightIndicator (Math|Rotator|MakeRotator (.roll _returnvalue_4) (.pitch (Transformation|GetWorldRotation FightIndicator)) (.yaw _returnvalue_4)) false false)
  (return))

(fn ConeAttackSAStartup
  (Rendering|SetVisibility (Variables|Default|GetSM_AI_SA_StartUp) true false)
  (Rendering|SetVisibility (Variables|Default|GetAttackStateIndicator) true false)
  (Rendering|Components|Decal|SetDecalMaterial (Variables|Default|GetAttackStateIndicator) "/Game/Assets/Materials/AI/M_AI_IsAttacking/M_AI_IsAttacking_Inst2.M_AI_IsAttacking_Inst2")
  (Components|Activation|Activate (Variables|Default|GetP_TA_Trails_1) true))