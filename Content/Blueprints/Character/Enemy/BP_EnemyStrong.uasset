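; Strong enemy character Blueprint that drives the visual, audio, camera and rumble feedback for its combat states.
; AnimBp_EnemyStrong dispatchers for its two attacks (SA cone, TA) switch decal indicators, trails and particles through startup, active and end phases.
; Hit, death, last-in-group death and fight-start events trigger camera shakes, effects or a camera-facing alert sign.
; Timelines animate scale pulses and drive hit-stop through global time dilation.
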(event Custom|TA_Startup_Event_0
  ;[1 1 1] On AI 3 Attack: Cone Attack & Tourbilol Attack
  (Rendering|SetVisibility (Variables|Default|GetAttackStateIndicator) true false)
  (Components|Activation|Activate (Variables|Default|GetP_TA_Trails_1) true)
  (Rendering|Components|Decal|SetDecalMaterial (Variables|Default|GetAttackStateIndicator) "/Game/Assets/Materials/AI/M_AI_IsAttacking/M_AI_IsAttacking_Inst2.M_AI_IsAttacking_Inst2"))

(event Custom|AI3_EndAttack
  ;[1 1 1] On AI 3 Attack: Cone Attack & Tourbilol Attack
  (Components|Activation|Deactivate (Variables|Default|GetP_TA_Trails_1))
  (Rendering|SetVisibility (Variables|Default|GetAttackStateIndicator) false false)
  (Game|Feedback|ClientStopForceFeedback (Game|GetPlayerController 0) "/Game/Assets/ControllerFeedback/FE_AI4_Attack.FE_AI4_Attack" "None"))

(event Custom|AI3_ConeAttack_Startup
  ;[1 1 1] On AI 3 Attack: Cone Attack & Tourbilol Attack
  (CallFunction|ConeAttackSAStartUp))

(event Custom|SA_Active_Event_0
  ;[1 1 1] On AI 3 Attack: Cone Attack & Tourbilol Attack
  (Game|Feedback|ClientPlayForceFeedback (Game|GetPlayerController 0) "/Game/Assets/ControllerFeedback/FE_AI4_Attack.FE_AI4_Attack" "None" true false false)
  (Rendering|SetVisibility (Variables|Default|GetSM_AI_SA_StartUp) false false)
  (Components|Activation|Activate (Variables|Default|GetP_AI_SA_Active) true)
  (Components|Activation|Deactivate (Variables|Default|GetP_TA_Trails_1))
  (Rendering|Components|Decal|SetDecalMaterial (Variables|Default|GetAttackStateIndicator) "/Game/Assets/Materials/AI/M_AI_IsAttacking/M_AI_IsAttacking_Inst3.M_AI_IsAttacking_Inst3")
  (bind _focusindicator_rescale (Timeline|Timeline_4 PlayFromStart)
    (:Update
      (Transformation|SetWorldScale3D (Variables|Default|GetAttackStateIndicator) (* _focusindicator_rescale (Variables|Default|GetattackStateIndicatorScale))))))

(event Custom|TA_Active_Event_0
  ;[1 1 1] On AI 3 Attack: Cone Attack & Tourbilol Attack
  (Rendering|Components|Decal|SetDecalMaterial (Variables|Default|GetAttackStateIndicator) "/Game/Assets/Materials/AI/M_AI_IsAttacking/M_AI_IsAttacking_Inst3.M_AI_IsAttacking_Inst3")
  (bind _focusindicator_rescale (Timeline|Timeline_4 PlayFromStart)
    (:Update
      (Transformation|SetWorldScale3D (Variables|Default|GetAttackStateIndicator) (* _focusindicator_rescale (Variables|Default|GetattackStateIndicatorScale))))))

(event EventBeginPlay
  ;[1 1 1] Set Current Weapon Size
  (Variables|Default|SetweaponScaleAtStart (Transformation|GetWorldScale (Variables|Default|GetSword02SM_1)))
  ;[1 1 1] Set Current Mesh Size
  (Variables|Default|SetmeshScaleAtStart (Transformation|GetWorldScale (Variables|Character|GetMesh)))
  ;[1 1 1] Get Character
  (bind _ascharacter_player (Utilities|Casting|CastToCharacter_Player (Game|GetPlayerCharacter 0)))
  (Variables|Default|SetPlayer _ascharacter_player)
  ;[1 1 1] Get Indicators Scales
  (Variables|Default|SetattackStateIndicatorScale (Transformation|GetWorldScale (Variables|Default|GetAttackStateIndicator)))
  (Variables|Default|SetfightIndicatorScale (Transformation|GetWorldScale (Variables|Default|GetFightIndicator)))
  ;[1 1 1] On AI 3 Attack: Cone Attack & Tourbilol Attack
  (bind _asanim_bp_enemy_strong (Utilities|Casting|CastToAnimBp_EnemyStrong (Components|SkeletalMesh|GetAnimInstance (Variables|Character|GetMesh))))
  (EventDispatchers|AssignSAStartup _asanim_bp_enemy_strong (delegate Custom|AI3_ConeAttack_Startup))
  (EventDispatchers|AssignTAStartup _asanim_bp_enemy_strong (delegate Custom|TA_Startup_Event_0))
  (EventDispatchers|AssignSAActive _asanim_bp_enemy_strong (delegate Custom|SA_Active_Event_0))
  (EventDispatchers|AssignTAActive _asanim_bp_enemy_strong (delegate Custom|TA_Active_Event_0))
  (EventDispatchers|AssignSAEnd _asanim_bp_enemy_strong (delegate Custom|AI3_EndAttack))
  (EventDispatchers|AssignTAEnd _asanim_bp_enemy_strong (delegate Custom|AI3_EndAttack)))

(event EventEnemyDeath
  ;[1 1 1] Enemy Strong Death
  (Utilities|ScreenShake "/Game/Blueprints/Character/BP_Shake_AI_Death.BP_Shake_AI_Death_C")
  (Rendering|SetVisibility (Variables|Default|GetAttackStateIndicator) false false)
  (Components|Activation|Deactivate (Variables|Default|GetP_TA_Trails_1))
  (Rendering|SetVisibility (Variables|Default|GetSM_AI_SA_StartUp) false false))

(event EventEnemyHitted
  (bind _meshscaleatstart (Variables|Default|GetmeshScaleAtStart))
  ;[1 1 1] CUSTOM EVENT: AI HasBeenHit
  (CallFunction|PlaySoundonHasBeenHit (Variables|Default|GetSE_AI_AsBeenHit))
  (Utilities|ScreenShake "/Game/Blueprints/Character/BP_Shake_AsBeenHit.BP_Shake_AsBeenHit_C")
  (bind _hitstop (Timeline|Timeline_0 PlayFromStart)
    (:Update
      (Utilities|HitStop _hitstop :!label _label)
      (Components|Activation|SetActive (Variables|Default|GetParticleBlood) true true)
      (bind _meshrescale (Timeline|Timeline_1 PlayFromStart)
        (:Update
          (Transformation|SetWorldScale3D (Variables|Character|GetMesh) (* _meshrescale _meshscaleatstart)))
        (:Finished
          (Transformation|SetWorldScale3D (Variables|Character|GetMesh) _meshscaleatstart))))
    (:Finished
      (goto _label Finished))))

(event EventLastEnemyinGroup
  ;[1 1 1] On Last AI Death of AIDirector
  (Utilities|ScreenShake "/Game/Blueprints/Character/BP_Shake_AI_LastDeath.BP_Shake_AI_LastDeath_C")
  (Rendering|SetVisibility (Variables|Default|GetAttackStateIndicator) false false)
  (Rendering|SetVisibility (Variables|Default|GetSM_AI_SA_StartUp) false false)
  (Components|Activation|Deactivate (Variables|Default|GetP_TA_Trails_1))
  (Utilities|ParticleFlashEffect 0.6 true (Variables|Default|GetParticleFlash))
  (bind _hitstop (Timeline|Timeline_2 PlayFromStart)
    (:Update
      (Utilities|HitStop _hitstop :!label _label))
    (:Finished
      (goto _label Finished))))

(event EventEnemyStartFight
  (bind _returnvalue (Transformation|GetActorLocation))
  (bind _fightindicator (Variables|Default|GetFightIndicator))
  ;[1 1 1] Fight Indicator : Surpise Sign
  (Rendering|SetVisibility _fightindicator true false)
  (Transformation|SetWorldLocation _fightindicator (Math|Vector|MakeVector (.x _returnvalue) (.y _returnvalue) (+ (.z _returnvalue) 3e+02)) false false)
  (bind _opacityovertime (Timeline|Timeline_3 PlayFromStart)
    (:Update
      (Transformation|SetWorldScale3D _fightindicator (Math|Vector|MakeVector (+ _opacityovertime 1.0) (+ _opacityovertime 1.0) (+ _opacityovertime 1.0)))
      (Class|WidgetComponent|SetTintColorandOpacity _fightindicator (Utilities|Struct|MakeLinearColor 1.0 0.166518 0.0 _opacityovertime))
      (CallFunction|WDGFightIndicatorRotation (Variables|Default|GetFightIndicator)))
    (:Finished
      (Rendering|SetVisibility _fightindicator false false))))

(fn ConstructionScript)

(fn PlaySoundonHasBeenHit
  (params (SE_HasBeenHit :type Audio%20Component%20Object%20Reference))
  (Audio|Components|Audio|SetPitchMultiplier SE_HasBeenHit (Math|Random|RandomFloatinRange 0.8 1.0))
  (Audio|Components|Audio|Stop SE_HasBeenHit)
  (Audio|Components|Audio|Play SE_HasBeenHit 0.0)
  (return))

(fn WDGFightIndicatorRotation
  (params (FightIndicator :type Scene%20Component%20Object%20Reference))
  (bind _returnvalue (Game|GetPlayerCameraManager 0))
  (bind _returnvalue_2 (Transformation|GetActorLocation))
  (bind _returnvalue_3 (Transformation|GetActorLocation _returnvalue))
  (bind _returnvalue_4 (Math|Rotator|FindLookatRotation _returnvalue_2 _returnvalue_3))
  (Transformation|SetWorldRotation FightIndicator (Math|Rotator|MakeRotator (.roll _returnvalue_4) (.pitch (Transformation|GetWorldRotation FightIndicator)) (.yaw _returnvalue_4)) false false)
  (return))

(fn ConeAttackSAStartup
  (Rendering|SetVisibility (Variables|Default|GetSM_AI_SA_StartUp) true false)
  (Rendering|SetVisibility (Variables|Default|GetAttackStateIndicator) true false)
  (Rendering|Components|Decal|SetDecalMaterial (Variables|Default|GetAttackStateIndicator) "/Game/Assets/Materials/AI/M_AI_IsAttacking/M_AI_IsAttacking_Inst2.M_AI_IsAttacking_Inst2")
  (Components|Activation|Activate (Variables|Default|GetP_TA_Trails_1) true))