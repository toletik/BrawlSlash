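; Weak shielded enemy Blueprint that handles combat feedback: shield material setup, hit reactions, attack warning and fight-start indicator.
; Hits trigger randomized-pitch sound, camera shake, blood particles and a mesh rescale pulse.
; Timelines drive hit stop through global time dilation on hits and on the group's last death, which adds a flash and clears attack visuals.
; The fight indicator scales, fades and turns toward the camera.
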(event Custom|EnemyStartNeedAttackWeak_1
  (bind _attackstateindicator (Variables|Default|GetAttackStateIndicator))
  ;[1 1 1] When Need To Attack (Weak Attack) : Attack Sign
  (Rendering|SetVisibility _attackstateindicator true false)
  (Rendering|Components|Decal|SetDecalMaterial _attackstateindicator "/Game/Assets/Materials/AI/M_AI_IsAttacking/M_AI_IsAttacking_Inst2.M_AI_IsAttacking_Inst2"))

(event EventBeginPlay
  (bind _shieldcomponent (Variables|Default|GetshieldComponent))
  ;[1 1 1] Set Current Shield Size
  (Variables|Default|SetshieldScaleAtStart (Transformation|GetWorldScale (Variables|/Script/BrawlSlash.Component_EnemyShield|GetshieldFront (Variables|Default|GetshieldComponent))))
  ;[1 1 1] Set Current Weapon Size
  (Variables|Default|SetweaponScaleAtStart (Transformation|GetWorldScale (Variables|Default|GetSword02SM_1)))
  ;[1 1 1] Set Current Mesh Size
  (Variables|Default|SetmeshScaleAtStart (Transformation|GetWorldScale (Variables|Character|GetMesh)))
  ;[1 1 1] Get Character
  (bind _ascharacter_player (Utilities|Casting|CastToCharacter_Player (Game|GetPlayerCharacter 0)))
  (Variables|Default|SetPlayer _ascharacter_player)
  ;[1 1 1] Get Indicators Scales
  (Variables|Default|SetattackStateIndicatorScale (Transformation|GetWorldScale (Variables|Default|GetAttackStateIndicator)))
  (Variables|Default|SetfightIndicatorScale (Transformation|GetWorldScale (Variables|Default|GetFightIndicator)))
  ;[0.9341 1 0.9301] Set Current Shield Active
  (if (Variables|/Script/BrawlSlash.Component_EnemyShield|GetisShieldInFront _shieldcomponent)
    (Rendering|Material|SetMaterial (Variables|/Script/BrawlSlash.Component_EnemyShield|GetshieldFront _shieldcomponent) 0 "/Game/Assets/Materials/AI/M_AI_Shield/M_AI_Shield_Inst.M_AI_Shield_Inst"))
  (if (Variables|/Script/BrawlSlash.Component_EnemyShield|GetisShieldInBack _shieldcomponent)
    (Rendering|Material|SetMaterial (Variables|/Script/BrawlSlash.Component_EnemyShield|GetshieldBack _shieldcomponent) 0 "/Game/Assets/Materials/AI/M_AI_Shield/M_AI_Shield_Inst.M_AI_Shield_Inst")))

(event EventEnemyHitted
  (bind _meshscaleatstart (Variables|Default|GetmeshScaleAtStart))
  ;[1 1 1] CUSTOM EVENT: AI HasBeenHit
  (CallFunction|PlaySoundonHasBeenHit (Variables|Default|GetSE_AI_AsBeenHit))
  (Utilities|ScreenShake "/Game/Blueprints/Character/BP_Shake_AsBeenHit.BP_Shake_AsBeenHit_C")
  (bind _hitstop (Timeline|Timeline_0 PlayFromStart)
    (:Update
      (Utilities|HitStop _hitstop :!label _label)
      (Components|Activation|SetActive (Variables|Default|GetParticleBlood) true true)
      (bind _meshrescale (Timeline|Timeline_1 PlayFromStart)
        (:Update
          (Transformation|SetWorldScale3D (Variables|Character|GetMesh) (* _meshrescale _meshscaleatstart)))
        (:Finished
          (Transformation|SetWorldScale3D (Variables|Character|GetMesh) _meshscaleatstart))))
    (:Finished
      (goto _label Finished))))

(event EventLastEnemyinGroup
  ;[1 1 1] On Last AI Death of AIDirector
  (Utilities|ScreenShake "/Game/Blueprints/Character/BP_Shake_AI_LastDeath.BP_Shake_AI_LastDeath_C")
  (Utilities|ParticleFlashEffect 0.6 true (Variables|Default|GetParticleFlash))
  (bind _hitstop (Timeline|Timeline_2 PlayFromStart)
    (:Update
      (Utilities|HitStop _hitstop :!label _label)
      (Rendering|SetVisibility (Variables|Default|GetAttackStateIndicator) false false)
      (Components|Activation|Deactivate (Variables|Default|GetP_TA_Trails_1)))
    (:Finished
      (goto _label Finished))))

(event EventEnemyStartFight
  (bind _returnvalue (Transformation|GetActorLocation))
  (bind _fightindicator (Variables|Default|GetFightIndicator))
  ;[1 1 1] Fight Indicator : Surpise Sign
  (Rendering|SetVisibility _fightindicator true false)
  (Transformation|SetWorldLocation _fightindicator (Math|Vector|MakeVector (.x _returnvalue) (.y _returnvalue) (+ (.z _returnvalue) 3e+02)) false false)
  (bind _opacityovertime (Timeline|Timeline_3 PlayFromStart)
    (:Update
      (Transformation|SetWorldScale3D _fightindicator (Math|Vector|MakeVector (+ _opacityovertime 1.0) (+ _opacityovertime 1.0) (+ _opacityovertime 1.0)))
      (Class|WidgetComponent|SetTintColorandOpacity _fightindicator (Utilities|Struct|MakeLinearColor 1.0 0.166518 0.0 _opacityovertime))
      (CallFunction|WDGFightIndicatorRotation (Variables|Default|GetFightIndicator)))
    (:Finished
      (Rendering|SetVisibility _fightindicator false false))))

(fn ConstructionScript)

(fn PlaySoundonHasBeenHit
  (params (SE_HasBeenHut :type Audio%20Component%20Object%20Reference))
  (Audio|Components|Audio|SetPitchMultiplier SE_HasBeenHut (Math|Random|RandomFloatinRange 0.8 1.0))
  (Audio|Components|Audio|Stop SE_HasBeenHut)
  (Audio|Components|Audio|Play SE_HasBeenHut 0.0)
  (return))

(fn WDGFightIndicatorRotation
  (params (FightIndicator :type Scene%20Component%20Object%20Reference))
  (bind _returnvalue (Game|GetPlayerCameraManager 0))
  (bind _returnvalue_2 (Transformation|GetActorLocation))
  (bind _returnvalue_3 (Transformation|GetActorLocation _returnvalue))
  (bind _returnvalue_4 (Math|Rotator|FindLookatRotation _returnvalue_2 _returnvalue_3))
  (Transformation|SetWorldRotation FightIndicator (Math|Rotator|MakeRotator (.roll _returnvalue_4) (.pitch (Transformation|GetWorldRotation FightIndicator)) (.yaw _returnvalue_4)) false false)
  (return))