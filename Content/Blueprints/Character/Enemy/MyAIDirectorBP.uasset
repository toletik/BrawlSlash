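; AI director that keeps cleared enemy groups from reappearing, using state stored in MyGameInstance.
; On BeginPlay it registers its UniqueIndex as active in the AllDirectors map, or, if already marked cleared, destroys its Enemies and itself.
; The all-enemies-dead event sets that map entry to false.
; Each of these state changes prints a colored debug message.
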(event EventBeginPlay
  (bind _asmy_game_instance (Utilities|Casting|CastToMyGameInstance (Game|GetGameInstance)))
  (if (Utilities|Map|Contains (Variables|/Script/BrawlSlash.MyGameInstance|GetallDirectors _asmy_game_instance) (Variables|Default|GetuniqueIndex))
    (if (not (.Value (Utilities|Map|Find (Variables|/Script/BrawlSlash.MyGameInstance|GetallDirectors _asmy_game_instance) (Variables|Default|GetuniqueIndex))))
      (for _array_element (Variables|Default|Getenemies)
        (Actor|DestroyActor _array_element))
      (Development|PrintString (Utilities|String|Append (Utilities|String|MakeLiteralString "Initial Supp : ") (Utilities|GetDisplayName self)) true true "(R=1.000000,G=0.000000,B=0.071264,A=1.000000)")
      (Actor|DestroyActor))
    (else
      (Utilities|Map|Add (Variables|/Script/BrawlSlash.MyGameInstance|GetallDirectors _asmy_game_instance) (Variables|Default|GetuniqueIndex) true)
      (Development|PrintString (Utilities|String|Append (Utilities|String|MakeLiteralString "Initial Add  : ") (Utilities|GetDisplayName self)) true true "(R=0.000000,G=1.000000,B=0.016302,A=1.000000)"))))

(event EventAIDirectorAllEnemiesDead
  (bind _asmy_game_instance (Utilities|Casting|CastToMyGameInstance (Game|GetGameInstance)))
  (Utilities|Map|Add (Variables|/Script/BrawlSlash.MyGameInstance|GetallDirectors _asmy_game_instance) (Variables|Default|GetuniqueIndex) false)
  (Development|PrintString (Utilities|String|Append (Utilities|String|MakeLiteralString "removed : ") (Utilities|GetDisplayName self)) true true "(R=1.000000,G=0.827031,B=0.000000,A=1.000000)"))

(fn ConstructionScript)