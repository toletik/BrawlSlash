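; Dummy enemy that plays combat feedback when hit, killed or last to die in an AI Director group.
; Each event triggers a camera shake and turns blood and flash particles according to whether the player is in front.
; Hits add pitch-randomized sound, timeline-driven hit stop through global time dilation, blood and a mesh scale pulse.
; Deaths fire a timed flash, with slow motion for the group's last and wood sound and blood otherwise.
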(event EventBeginPlay
  ;[1 1 1] Set Current Mesh Size
  (Variables|Default|SetmeshScaleAtStart (Transformation|GetWorldScale (Variables|Character|GetMesh)))
  ;[1 1 1] Get Character
  (bind _ascharacter_player (Utilities|Casting|CastToCharacter_Player (Game|GetPlayerCharacter 0)))
  (Variables|Default|SetPlayer _ascharacter_player))

(event EventEnemyHitted
  (bind _meshscaleatstart (Variables|Default|GetmeshScaleAtStart))
  ;[1 1 1] CUSTOM EVENT: AI HasBeenHit
  (CallFunction|PlaySoundonHasBeenHit (Variables|Default|GetSE_AI_AsBeenHit))
  (CallFunction|RotateParticles)
  (Utilities|ScreenShake "/Game/Blueprints/Character/BP_Shake_AsBeenHit.BP_Shake_AsBeenHit_C")
  (bind _hitstop (Timeline|Timeline_0 PlayFromStart)
    (:Update
      (Utilities|HitStop _hitstop :!label _label)
      (Components|Activation|SetActive (Variables|Default|GetParticleBlood) true true)
      (bind _meshrescale (Timeline|Timeline_1 PlayFromStart)
        (:Update
          (Transformation|SetWorldScale3D (Variables|Character|GetMesh) (* _meshrescale _meshscaleatstart)))
        (:Finished
          (Transformation|SetWorldScale3D (Variables|Character|GetMesh) _meshscaleatstart))))
    (:Finished
      (goto _label Finished))))

(event EventLastEnemyinGroup
  ;[1 1 1] On Last AI Death of AIDirector
  (Utilities|ScreenShake "/Game/Blueprints/Character/BP_Shake_AI_LastDeath.BP_Shake_AI_LastDeath_C")
  (CallFunction|RotateParticles)
  (Utilities|ParticleFlashEffect 0.6 true (Variables|Default|GetParticleFlash))
  (bind _hitstop (Timeline|Timeline_2 PlayFromStart)
    (:Update
      (Utilities|HitStop _hitstop :!label _label))
    (:Finished
      (goto _label Finished))))

(event EventEnemyDeath
  ;[1 1 1] Dummy Death
  (Utilities|ScreenShake "/Game/Blueprints/Character/BP_Shake_AI_LastDeath.BP_Shake_AI_LastDeath_C")
  (CallFunction|RotateParticles)
  (Utilities|ParticleFlashEffect 0.1 true (Variables|Default|GetParticleFlash))
  (Audio|PlaySound2D "/Game/Assets/Sounds/LDBricks/SE_WoodHit.SE_WoodHit" 1.0 1.0 0.0 0 0)
  (Components|Activation|SetActive (Variables|Default|GetParticleBlood) true true))

(fn ConstructionScript)

(fn PlaySoundonHasBeenHit
  (params (SE_HasBeenHit :type Audio%20Component%20Object%20Reference))
  (Audio|Components|Audio|SetPitchMultiplier SE_HasBeenHit (Math|Random|RandomFloatinRange 0.8 1.0))
  (Audio|Components|Audio|Stop SE_HasBeenHit)
  (Audio|Components|Audio|Play SE_HasBeenHit 0.0)
  (return))

(fn RotateParticles
  (bind _particleblood (Variables|Default|GetParticleBlood))
  (bind _particleflash (Variables|Default|GetParticleFlash))
  (bind _returnvalue (Class|CharacterEnemyBase|IsPlayerinFront (Transformation|GetActorLocation (Variables|Default|GetPlayer))))
  (if _returnvalue
    (Transformation|SetRelativeRotation _particleblood "110.000000, 0, 0" false false)
    (Transformation|SetRelativeRotation _particleflash "180.000000, 0, 0" false false)
    (return)
    (else
      (Transformation|SetRelativeRotation _particleblood "-70.000000, 0, 0" false false)
      (Transformation|SetRelativeRotation _particleflash "0, 0, 0" false false))))