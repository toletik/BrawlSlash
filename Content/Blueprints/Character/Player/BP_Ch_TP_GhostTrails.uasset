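; Third-person player ghost trail actor that shows a frozen afterimage of the player character's pose.
; On BeginPlay it gives each poseable mesh material slot a dynamic instance, copies the pose from the player's skeletal mesh and starts the Opacity timeline.
; The timeline is set up to feed a scalar material parameter, whose name is left as None, and destroy the actor when finished.
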(event Custom|GhostTrails
  (for _array_element (Rendering|Material|GetMaterials (Variables|Default|GetPoseableMesh))
    (bind _returnvalue (Rendering|Material|CreateDynamicMaterialInstance "/Game/Assets/Materials/Character/M_Ch_TP/M_Ch_TP_Inst.M_Ch_TP_Inst" "None" :!class /Script/Engine.KismetMaterialLibrary))
    (bind _returnvalue_2 (Utilities|Array|Add (Variables|Default|GetDynamicMats) _returnvalue))
    (Rendering|Material|SetMaterial (Variables|Default|GetPoseableMesh) _returnvalue_2 _returnvalue)
    (Class|PoseableMeshComponent|CopyPosefromSkeletalComponent (Variables|Default|GetPoseableMesh) (Variables|/Script/Engine.Character|GetMesh (Variables|Default|GetPlayerCharacterRef)))
    (Components|Timeline|PlayfromStart (Variables|Colors|GetOpacity))))

(event EventBeginPlay
  (bind _asmy_character_player (Utilities|Casting|CastToMyCharacter_Player (Game|Player|GetPlayerPawn 0)))
  (Variables|Default|SetPlayerCharacterRef _asmy_character_player)
  (CallFunction|GhostTrails))

(fn ConstructionScript)