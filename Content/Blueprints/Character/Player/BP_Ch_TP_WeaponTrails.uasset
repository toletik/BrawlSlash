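; Short-lived weapon trail actor that leaves a static mesh copy at the pose of the player's sword.
; On BeginPlay it casts the first player pawn to MyCharacter_Player and snaps its StaticMesh once to the world location and rotation of Sword02SM.
; The mesh does not follow the sword afterwards, and the actor destroys itself after a brief delay.
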(event Custom|WeaponTrails
  (bind _staticmesh (Variables|Default|GetStaticMesh))
  (bind _playercharacterref (Variables|Default|GetPlayerCharacterRef))
  (bind _sword02sm (Variables|/Game/Blueprints/Character/Player/MyCharacter_Player.MyCharacter_Player_C|GetSword02SM _playercharacterref))
  (Transformation|SetWorldLocation _staticmesh (Transformation|GetWorldLocation _sword02sm) false false)
  (Transformation|SetWorldRotation _staticmesh (Transformation|GetWorldRotation _sword02sm) false false)
  (Utilities|FlowControl|Delay 0.2)
  (Actor|DestroyActor))

(event EventBeginPlay
  (bind _asmy_character_player (Utilities|Casting|CastToMyCharacter_Player (Game|Player|GetPlayerPawn 0)))
  (Variables|Default|SetPlayerCharacterRef _asmy_character_player)
  (CallFunction|WeaponTrails))

(fn ConstructionScript)