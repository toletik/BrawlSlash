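; BP_SequenceMenu drives the main menu's level sequences and the hand-off to the lobby map.
; On BeginPlay it stops the any-key sequence, shows the main menu widget with the mouse cursor and binds its OnIntro and OnStart dispatchers.
; OnIntro plays the loop sequence; OnStart swaps to the start sequence, replaces widgets with a fade-in and opens Map_Lobby after a delay.
; The intro sequence's Play call is unconnected.
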(event Custom|OnIntro_Event_0
  (Sequencer|Player|Play (Variables|/Script/LevelSequence.LevelSequenceActor|GetSequencePlayer (Variables|Default|GetLevelSequence_Loop)) :!class /Script/MovieScene.MovieSceneSequencePlayer))

(event Custom|FinishIntro)

(event Custom|OnStart
  (Sequencer|Player|Stop (Variables|/Script/LevelSequence.LevelSequenceActor|GetSequencePlayer (Variables|Default|GetLevelSequence_Intro)) :!class /Script/MovieScene.MovieSceneSequencePlayer)
  (Sequencer|Player|Stop (Variables|/Script/LevelSequence.LevelSequenceActor|GetSequencePlayer (Variables|Default|GetLevelSequence_Loop)) :!class /Script/MovieScene.MovieSceneSequencePlayer)
  (Sequencer|Player|Play (Variables|/Script/LevelSequence.LevelSequenceActor|GetSequencePlayer (Variables|Default|GetLevelSequence_Start)) :!class /Script/MovieScene.MovieSceneSequencePlayer)
  (Viewport|RemoveAllWidgets)
  (bind _returnvalue (UserInterface|CreateWidget "/Game/Blueprints/UI/WDG_FadeIn.WDG_FadeIn_C" (Game|GetPlayerController 0)))
  (UserInterface|Viewport|AddtoViewport _returnvalue 0)
  (Utilities|FlowControl|Delay 2.0)
  (Game|OpenLevel(byName) "Map_Lobby"))

(event EventBeginPlay
  (Sequencer|Player|Stop (Variables|/Script/LevelSequence.LevelSequenceActor|GetSequencePlayer (Variables|Default|GetLevelSequence_AnyKey)) :!class /Script/MovieScene.MovieSceneSequencePlayer)
  (bind _returnvalue (UserInterface|CreateWidget "/Game/Blueprints/UI/WDG_MainMenu.WDG_MainMenu_C"))
  (Variables|Default|SetWDG_MainMenu _returnvalue)
  (UserInterface|Viewport|AddtoViewport (Variables|Default|GetWDG_MainMenu) 0)
  (Variables|/Script/Engine.PlayerController|SetbShowMouseCursor (Game|GetPlayerController 0) true)
  (EventDispatchers|AssignOnStart (Variables|Default|GetWDG_MainMenu) (delegate Custom|OnStart))
  (EventDispatchers|AssignOnIntro (Variables|Default|GetWDG_MainMenu) (delegate Custom|OnIntro_Event_0)))

(fn ConstructionScript)