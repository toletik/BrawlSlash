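; BP_Door is a breakable door that takes damage when the player's attack box overlaps its poles mesh.
; Each hit subtracts the player's damage from Hp, plays a sound, and pulses the boards' scale through a timeline based on the poles' initial scale.
; At zero Hp, a short delay precedes break particles and destruction of only the boards component.
; A separate function tints a focus widget by short-range focus state.
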(event OnComponentBeginOverlap(SM_Door_Poles)
  (params (OverlappedComponent :type Primitive%20Component%20Object%20Reference) (OtherActor :type Actor%20Object%20Reference) (OtherComp :type Primitive%20Component%20Object%20Reference) (OtherBodyIndex :type Integer) (bFromSweep :type Boolean) (SweepResult :type Hit%20Result%20Structure%20%28by%20ref%29))
  (bind _se_hit (Variables|Default|GetSE_Hit))
  (bind _player (Variables|Player|GetPlayer))
  ;[1 1 1] On Attacked By Player
  (if (== OtherComp (Variables|/Script/BrawlSlash.Character_Base|GetattackBox _player))
    (bind _output_get (Variables|Focusable|SetHp (- (Variables|Focusable|GetHp) (Variables|/Script/BrawlSlash.Character_Base|GettoDoDamage _player))))
    (if (> _output_get 0)
      ;[1 1 1] On Player Hit
      (Audio|Components|Audio|Stop _se_hit)
      (Audio|Components|Audio|Play _se_hit 0.0)
      (bind _focusindicator (Timeline|Timeline_1 PlayFromStart)
        (:Update
          (Transformation|SetWorldScale3D (Variables|Default|GetSM_DoorBoards) (* _focusindicator (Variables|Mesh|GetmeshScale)))))
      (else
        ;[1 1 1] On Break
        (if (Utilities|IsValid (Variables|Default|GetSM_DoorBoards))
          (Audio|Components|Audio|Stop (Variables|Default|GetSE_Hit))
          (Audio|Components|Audio|Play (Variables|Default|GetSE_Hit) 0.0)
          (Utilities|FlowControl|Delay 0.2)
          (Components|Activation|Activate (Variables|Default|GetP_Break) false)
          (Components|DestroyComponent (Variables|Default|GetSM_DoorBoards)))))))

(event EventBeginPlay
  ;[1 1 1] Setting Var
  (bind _ascharacter_player (Utilities|Casting|CastToCharacter_Player (Game|GetPlayerCharacter 0)))
  (Variables|Player|SetPlayer _ascharacter_player)
  ;;[1 1 1] Get Indicators Scales
  (Variables|Mesh|SetmeshScale (Transformation|GetWorldScale (Variables|Default|GetSM_Door_Poles))))

(fn ConstructionScript)

(fn FocusIndicatorColorisation
  (params (widgetFocusIndicator :type Widget%20Component%20Object%20Reference))
  (if (Variables|/Script/BrawlSlash.Character_Player|GetisFocusInShortRange (Variables|Player|GetPlayer))
    (if (not (LocalVariables|GetcoloredShort))
      (Class|WidgetComponent|SetTintColorandOpacity widgetFocusIndicator "(R=0.218442,G=0.649466,B=0.713542,A=1.000000)")
      (LocalVariables|SetcoloredShort true))
    (elif (LocalVariables|GetcoloredShort)
      (Class|WidgetComponent|SetTintColorandOpacity widgetFocusIndicator "(R=0.671088,G=0.678770,B=0.744792,A=1.000000)")
      (LocalVariables|SetcoloredShort false))))