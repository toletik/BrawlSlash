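; SafeZone is a level-design trigger volume that ends the player's current enemy fight when they enter it.
; Cube overlap events filter for the Character_Player capsule component.
; On entry it calls SetEndToFight on the player's CurrentEnemyGroup, if one is set.
; Both entry and exit set IsInSafeZone to false, so this Blueprint never marks the player as safe.
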(event OnComponentEndOverlap(Cube)
  (params (OverlappedComponent :type Primitive%20Component%20Object%20Reference) (OtherActor :type Actor%20Object%20Reference) (OtherComp :type Primitive%20Component%20Object%20Reference) (OtherBodyIndex :type Integer))
  (bind _ascharacter_player (Utilities|Casting|CastToCharacter_Player OtherActor))
  (if (== OtherComp (Variables|/Script/Engine.Character|GetCapsuleComponent _ascharacter_player))
    (Variables|/Script/BrawlSlash.Character_Player|SetisInSafeZone _ascharacter_player false)))

(event OnComponentBeginOverlap(Cube)
  (params (OverlappedComponent :type Primitive%20Component%20Object%20Reference) (OtherActor :type Actor%20Object%20Reference) (OtherComp :type Primitive%20Component%20Object%20Reference) (OtherBodyIndex :type Integer) (bFromSweep :type Boolean) (SweepResult :type Hit%20Result%20Structure%20%28by%20ref%29))
  (bind _ascharacter_player (Utilities|Casting|CastToCharacter_Player OtherActor))
  (if (== OtherComp (Variables|/Script/Engine.Character|GetCapsuleComponent _ascharacter_player))
    (Variables|/Script/BrawlSlash.Character_Player|SetisInSafeZone _ascharacter_player false)
    (if (!= (Variables|/Script/BrawlSlash.Character_Player|GetcurrentEnemyGroup _ascharacter_player) 0)
      (Class|MyAIDirector|SetEndtoFight (Variables|/Script/BrawlSlash.Character_Player|GetcurrentEnemyGroup _ascharacter_player)))))

(fn ConstructionScript)