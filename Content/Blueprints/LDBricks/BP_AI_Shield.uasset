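; BP_AI_Shield is an AI shield level-design brick that shows state changes and hit feedback.
; State events toggle the shield mesh's visibility for active or inactive and swap to a second material instance during either transition.
; On a hit, it plays a sound if not already playing, briefly activates a particle effect, and runs a timeline that rescales the mesh before restoring unit scale.
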(event Custom|IsActive
  (bind _sm_ai_shield (Variables|Default|GetSM_AI_Shield))
  ;[1 1 1] On Active
  (Rendering|Material|SetMaterial (Variables|Default|GetSM_AI_Shield) 0 "/Game/Assets/Materials/AI/M_AI_Shield/M_AI_Shield_Inst.M_AI_Shield_Inst")
  (if (not (Rendering|IsVisible _sm_ai_shield))
    (Rendering|SetVisibility _sm_ai_shield true false)))

(event Custom|IsNotActive
  (bind _sm_ai_shield (Variables|Default|GetSM_AI_Shield))
  ;[1 1 1] On Inactive
  (Rendering|Material|SetMaterial (Variables|Default|GetSM_AI_Shield) 0 "/Game/Assets/Materials/AI/M_AI_Shield/M_AI_Shield_Inst.M_AI_Shield_Inst")
  (if (Rendering|IsVisible _sm_ai_shield)
    (Rendering|SetVisibility _sm_ai_shield false false)))

(event Custom|IsTransitionningToActive
  ;[1 1 1] On IsTransitionningToActive
  (Rendering|Material|SetMaterial (Variables|Default|GetSM_AI_Shield) 0 "/Game/Assets/Materials/AI/M_AI_Shield/M_AI_Shield_Inst_2.M_AI_Shield_Inst_2"))

(event Custom|IsTransitionningToInactive
  ;[1 1 1] On IsTransitionningToInactive
  (Rendering|Material|SetMaterial (Variables|Default|GetSM_AI_Shield) 0 "/Game/Assets/Materials/AI/M_AI_Shield/M_AI_Shield_Inst_2.M_AI_Shield_Inst_2"))

(event Custom|IsHitted
  (bind _particlehitshield (Variables|Default|GetParticleHitShield))
  (bind _se_hitshield (Variables|Default|GetSE_HitShield))
  ;[1 1 1] On HitShield
  (Utilities|FlowControl|Sequence
    (:then_0
      ;;[1 1 1] SoundEffect
      (if (not (Audio|Components|Audio|IsPlaying _se_hitshield))
        (Audio|Components|Audio|Play _se_hitshield 0.0)))
    (:then_1
      ;;[1 1 1] Particle
      (Components|Activation|Activate _particlehitshield false)
      (Utilities|FlowControl|Delay 0.3)
      (Components|Activation|Deactivate _particlehitshield))
    (:then_2
      ;;[1 1 1] Shield ReScale
      (bind _shieldscale (Timeline|reScale Play)
        (:Update
          (Transformation|SetWorldScale3D (Variables|Default|GetSM_AI_Shield) _shieldscale))
        (:Finished
          (Transformation|SetWorldScale3D (Variables|Default|GetSM_AI_Shield) "1.000000,1.000000,1.000000"))))))

(event EventTick
  (params (DeltaSeconds :type Float%20%28single-precision%29)))

(fn ConstructionScript)