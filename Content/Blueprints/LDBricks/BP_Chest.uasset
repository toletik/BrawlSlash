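; Breakable level chest that the player damages to release a BP_HealthMaxPoints pickup.
; Overlaps with the player's attack box and capsule hits during a dash hit subtract the player's damage from Hp.
; Surviving hits play a sound and a timeline scale effect; breaking plays the sound, then after a short delay triggers particles, spawns the pickup and destroys the mesh component.
; A helper function tints a focus indicator widget by short-range focus state.
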(event OnComponentBeginOverlap(SM_Chest)
  (params (OverlappedComponent :type Primitive%20Component%20Object%20Reference) (OtherActor :type Actor%20Object%20Reference) (OtherComp :type Primitive%20Component%20Object%20Reference) (OtherBodyIndex :type Integer) (bFromSweep :type Boolean) (SweepResult :type Hit%20Result%20Structure%20%28by%20ref%29))
  (bind _se_hit (Variables|Default|GetSE_Hit))
  (bind _player (Variables|Player|GetPlayer))
  (bind _sm_chest (Variables|Default|GetSM_Chest))
  (bind _returnvalue (Transformation|GetWorldLocation _sm_chest))
  ;[1 1 1] On Attacked By Player
  (if (== OtherComp (Variables|/Script/BrawlSlash.Character_Base|GetattackBox _player))
    (bind _output_get (Variables|Focus|SetHp (- (Variables|Focus|GetHp) (Variables|/Script/BrawlSlash.Character_Base|GettoDoDamage _player))))
    (if (> _output_get 0)
      ;[1 1 1] On Hit
      (Audio|Components|Audio|Stop _se_hit)
      (Audio|Components|Audio|Play _se_hit 0.0)
      (bind _focusindicator (Timeline|TL_RescaleMesh PlayFromStart)
        (:Update
          (Transformation|SetWorldScale3D (Variables|Default|GetSM_Chest) (* _focusindicator (Variables|Mesh|GetmeshScale)))))
      (else
        ;[1 1 1] On Break
        (Audio|Components|Audio|Stop (Variables|Default|GetSE_Hit))
        (Audio|Components|Audio|Play (Variables|Default|GetSE_Hit) 0.0)
        (Utilities|FlowControl|Delay 0.2)
        (Components|Activation|Activate (Variables|Default|GetParticleChest) false)
        (Game|SpawnActorfromClass "/Game/Blueprints/LDBricks/BP_HealthMaxPoints.BP_HealthMaxPoints_C" (Math|Transform|MakeTransform (Math|Vector|MakeVector (.x _returnvalue) (.y _returnvalue) (+ (.z _returnvalue) 7e+01)) "0, 0, 0" "0.500000,0.500000,0.500000") "Undefined" 0 0)
        (Components|DestroyComponent (Variables|Default|GetSM_Chest))))))

(event OnComponentHit(SM_Chest)
  (params (HitComponent :type Primitive%20Component%20Object%20Reference) (OtherActor :type Actor%20Object%20Reference) (OtherComp :type Primitive%20Component%20Object%20Reference) (NormalImpulse :type Vector :default "0, 0, 0") (Hit :type Hit%20Result%20Structure%20%28by%20ref%29))
  (bind _se_hit (Variables|Default|GetSE_Hit))
  (bind _player (Variables|Player|GetPlayer))
  (bind _sm_chest (Variables|Default|GetSM_Chest))
  (bind _returnvalue (Transformation|GetWorldLocation _sm_chest))
  ;[1 1 1] On Player Dash Hit
  (if (and (== OtherComp (Variables|/Script/Engine.Character|GetCapsuleComponent _player)) (Utilities|Enum|Equal(Enum) (Variables|/Script/BrawlSlash.Character_Base|Getstate _player) "DASHING_HIT"))
    (Class|CharacterPlayer|StopDashHit _player)
    (bind _output_get (Variables|Focus|SetHp (- (Variables|Focus|GetHp) (Variables|/Script/BrawlSlash.Character_Base|GettoDoDamage _player))))
    (if (> _output_get 0)
      ;[1 1 1] On Hit
      (Audio|Components|Audio|Stop _se_hit)
      (Audio|Components|Audio|Play _se_hit 0.0)
      (bind _focusindicator (Timeline|TL_RescaleMesh PlayFromStart)
        (:Update
          (Transformation|SetWorldScale3D (Variables|Default|GetSM_Chest) (* _focusindicator (Variables|Mesh|GetmeshScale)))))
      (else
        ;[1 1 1] On Break
        (Audio|Components|Audio|Stop (Variables|Default|GetSE_Hit))
        (Audio|Components|Audio|Play (Variables|Default|GetSE_Hit) 0.0)
        (Utilities|FlowControl|Delay 0.2)
        (Components|Activation|Activate (Variables|Default|GetParticleChest) false)
        (Game|SpawnActorfromClass "/Game/Blueprints/LDBricks/BP_HealthMaxPoints.BP_HealthMaxPoints_C" (Math|Transform|MakeTransform (Math|Vector|MakeVector (.x _returnvalue) (.y _returnvalue) (+ (.z _returnvalue) 7e+01)) "0, 0, 0" "0.500000,0.500000,0.500000") "Undefined" 0 0)
        (Components|DestroyComponent (Variables|Default|GetSM_Chest))))))

(event EventBeginPlay
  ;[1 1 1] Setting Var
  (bind _ascharacter_player (Utilities|Casting|CastToCharacter_Player (Game|GetPlayerCharacter 0)))
  (Variables|Player|SetPlayer _ascharacter_player)
  ;;[1 1 1] Get Indicators Scales
  (Variables|Mesh|SetmeshScale (Transformation|GetWorldScale (Variables|Default|GetSM_Chest))))

(fn ConstructionScript)

(fn FocusIndicatorColorisation
  (params (widgetFocusIndicator :type Widget%20Component%20Object%20Reference))
  (if (Variables|/Script/BrawlSlash.Character_Player|GetisFocusInShortRange (Variables|Player|GetPlayer))
    (if (not (LocalVariables|GetcoloredShort))
      (Class|WidgetComponent|SetTintColorandOpacity widgetFocusIndicator "(R=0.218442,G=0.649466,B=0.713542,A=1.000000)")
      (LocalVariables|SetcoloredShort true))
    (elif (LocalVariables|GetcoloredShort)
      (Class|WidgetComponent|SetTintColorandOpacity widgetFocusIndicator "(R=0.671088,G=0.678770,B=0.744792,A=1.000000)")
      (LocalVariables|SetcoloredShort false))))