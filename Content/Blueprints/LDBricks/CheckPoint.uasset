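; CheckPoint is a level design brick that records the player's respawn point when touched.
; When the player character's capsule overlaps its Cube, it writes its own location and a RotationForRespawn value to MyGameInstance and flags that a checkpoint has been taken.
; The actor stays in place afterwards, as its DestroyActor call is never run.
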(event OnComponentBeginOverlap(Cube)
  (params (OverlappedComponent :type Primitive%20Component%20Object%20Reference) (OtherActor :type Actor%20Object%20Reference) (OtherComp :type Primitive%20Component%20Object%20Reference) (OtherBodyIndex :type Integer) (bFromSweep :type Boolean) (SweepResult :type Hit%20Result%20Structure%20%28by%20ref%29))
  (bind _ascharacter_player (Utilities|Casting|CastToCharacter_Player OtherActor))
  (if (== OtherComp (Variables|/Script/Engine.Character|GetCapsuleComponent _ascharacter_player))
    (bind _asmy_game_instance (Utilities|Casting|CastToMyGameInstance (Game|GetGameInstance)))
    (Variables|/Script/BrawlSlash.MyGameInstance|SetlastCheckPointPos _asmy_game_instance (Transformation|GetActorLocation))
    (Variables|/Script/BrawlSlash.MyGameInstance|SetlastCheckPointRot _asmy_game_instance (Variables|Default|GetrotationForRespawn))
    (Variables|/Script/BrawlSlash.MyGameInstance|SethasTakenACheckpoint _asmy_game_instance true)))

(fn ConstructionScript)