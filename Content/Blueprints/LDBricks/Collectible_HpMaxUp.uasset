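; Collectible pickup that permanently raises the player's maximum health when touched.
; It spins by a fixed rotation step every tick, independent of delta time.
; When its Sphere overlaps a Character_Player's capsule component, it adds HpMaxUp to MaxHealth and destroys itself.
; Only MaxHealth changes, and overlaps from the player's other components are ignored.
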(event OnComponentBeginOverlap(Sphere)
  (params (OverlappedComponent :type Primitive%20Component%20Object%20Reference) (OtherActor :type Actor%20Object%20Reference) (OtherComp :type Primitive%20Component%20Object%20Reference) (OtherBodyIndex :type Integer) (bFromSweep :type Boolean) (SweepResult :type Hit%20Result%20Structure%20%28by%20ref%29))
  (bind _ascharacter_player (Utilities|Casting|CastToCharacter_Player OtherActor))
  (if (== (Variables|/Script/Engine.Character|GetCapsuleComponent _ascharacter_player) OtherComp)
    (Variables|/Script/BrawlSlash.Character_Base|SetmaxHealth _ascharacter_player (+ (Variables|/Script/BrawlSlash.Character_Base|GetmaxHealth _ascharacter_player) (Variables|Default|GethpMaxUp)))
    (Actor|DestroyActor)))

(event EventTick
  (params (DeltaSeconds :type Float%20%28single-precision%29))
  (Transformation|AddActorLocalRotation "0,5.000000, 0" false false))

(fn ConstructionScript)