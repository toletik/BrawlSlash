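; BP_ShieldPoints is a shield point pickup actor that reacts when the player touches it.
; On spawn, the HealthIncrease timeline moves it by adding a curve offset to its current location each update.
; Overlap of the player's capsule with SphereOutside plays a sound, scales the sphere and destroys the actor, with no shield value changed here.
; HighLightTarget swaps target materials, but its constant false condition only allows restoring the original.
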(event OnComponentBeginOverlap(SphereOutside)
  (params (OverlappedComponent :type Primitive%20Component%20Object%20Reference) (OtherActor :type Actor%20Object%20Reference) (OtherComp :type Primitive%20Component%20Object%20Reference) (OtherBodyIndex :type Integer) (bFromSweep :type Boolean) (SweepResult :type Hit%20Result%20Structure%20%28by%20ref%29))
  ;[1 1 1] On Overlap
  (bind _ascharacter_player (Utilities|Casting|CastToCharacter_Player OtherActor))
  (if (== OtherComp (Variables|/Script/Engine.Character|GetCapsuleComponent _ascharacter_player))
    (Audio|PlaySoundatLocation "/Game/Assets/Sounds/LDBricks/SE_ShieldPoint.SE_ShieldPoint" (Transformation|GetWorldLocation (Variables|Default|GetHealthsPoint)) "0, 0, 0" 1.0 1.0 0.0 0 0 0)
    (bind _scale (Timeline|Scale PlayFromStart)
      (:Update
        (Transformation|SetRelativeScale3D (Variables|Default|GetSphereOutside) _scale))
      (:Finished
        (Actor|DestroyActor)))))

(event EventBeginPlay
  (bind _returnvalue (Transformation|GetActorLocation))
  ;[1 1 1] Get Initials Values
  (bind _ascharacter_player (Utilities|Casting|CastToCharacter_Player (Game|GetPlayerCharacter 0)))
  (Variables|Player|Setplayer _ascharacter_player)
  (Variables|MaterialManagment|SetoldMaterial (Rendering|Material|GetMaterial (Variables|Default|GetSphereOutside) 0))
  (Variables|Default|SetInitialLocation _returnvalue)
  (bind _transform_movment_when_spawning (Timeline|Health%20increase PlayFromStart)
    (:Update
      (Transformation|SetActorLocation (+ _returnvalue _transform_movment_when_spawning) false false))))

(fn ConstructionScript)

(fn HighLightTarget
  (if false
    (if (not (Variables|Target|GetisHiglighted))
      (Rendering|Material|SetMaterial (Variables|Default|GetSphereOutside) 0 "/Game/Assets/Materials/LDBricks/M_LDBricks_IsTarget_Inst.M_LDBricks_IsTarget_Inst")
      (Variables|Target|SetisHiglighted true))
    (elif (Variables|Target|GetisHiglighted)
      (Rendering|Material|SetMaterial (Variables|Default|GetSphereOutside) 0 (Variables|MaterialManagment|GetoldMaterial))
      (Variables|Target|SetisHiglighted false))))