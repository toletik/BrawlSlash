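; BP_StackPoint is a floating sphere point that reacts when it becomes the player's Focus.
; Each Tick it toggles FocusIndicator with focus and disables the sphere's collision while focused, with nothing here re-enabling it.
; A Timeline restarted from Tick bobs the sphere around StartMove with an absolute sine of game time and zeroes Plasma position parameters.
; Target highlighting is hard-wired off, and the focus flash is unconnected.
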(event EventBeginPlay
  ;[1 1 1] Get Initials Values
  (bind _ascharacter_player (Utilities|Casting|CastToCharacter_Player (Game|GetPlayerCharacter 0)))
  (Variables|Player|Setplayer _ascharacter_player)
  (Variables|MaterialManagment|SetoldMaterial (Rendering|Material|GetMaterial (Variables|Default|GetSphereOutside) 0)))

(event EventTick
  (params (DeltaSeconds :type Float%20%28single-precision%29))
  (bind _startmove (Variables|Default|GetStartMove))
  (bind _plasma (Variables|Default|GetPlasma))
  (bind _returnvalue (Transformation|GetWorldLocation _startmove))
  (bind _returnvalue_2 (Transformation|GetWorldLocation _startmove))
  ;[1 1 1] Set HighLight ; Set Focus
  (Utilities|FlowControl|Sequence
    (:then_0
      (CallFunction|HighLightTarget))
    (:then_1
      (CallFunction|FocusIndicatorManagement))
    (:then_2
      (if (== (Variables|/Script/BrawlSlash.Character_Player|Getfocus (Variables|Player|Getplayer)) self)
        (Collision|SetCollisionEnabled (Variables|Default|GetSphereOutside) "NoCollision")))
    (:then_3
      (Timeline|Timeline_0 Play
        (:Update
          (Transformation|SetWorldLocation (Variables|Default|GetSphereOutside) (Math|Vector|Lerp(Vector) (Math|Vector|MakeVector (.x _returnvalue_2) (.y _returnvalue_2) (+ (.z _returnvalue_2) 1e+01)) (Math|Vector|MakeVector (.x _returnvalue) (.y _returnvalue) (+ (.z _returnvalue) -1e+01)) (Math|Float|Absolute(Float) (Math|Trig|Sin(Radians) (* (Utilities|Time|GetTimeSeconds) (Variables|Default|GetSpeedMove))))) false false)
          (Effects|Components|ParticleSystem|SetVectorParameter _plasma "Module.CenterPosition" "0, 0, 0")
          (Effects|Components|ParticleSystem|SetVectorParameter _plasma "Particles.Position" "0, 0, 0"))))))

(fn ConstructionScript)

(fn HighLightTarget
  (if false
    (if (not (Variables|Target|GetisHiglighted))
      (Rendering|Material|SetMaterial (Variables|Default|GetSphereOutside) 0 "/Game/Assets/Materials/LDBricks/M_LDBricks_IsTarget_Inst.M_LDBricks_IsTarget_Inst")
      (Variables|Target|SetisHiglighted true))
    (elif (Variables|Target|GetisHiglighted)
      (Rendering|Material|SetMaterial (Variables|Default|GetSphereOutside) 0 (Variables|MaterialManagment|GetoldMaterial))
      (Variables|Target|SetisHiglighted false))))

(fn FocusIndicatorManagement
  (if (== (Variables|/Script/BrawlSlash.Character_Player|Getfocus (Variables|Player|Getplayer)) self)
    ;[1 1 1] On AI Focus by Character
    (if (not (Variables|Focus|GetisFocussed))
      (Rendering|SetVisibility (Variables|Default|GetFocusIndicator) true false)
      (Variables|Focus|SetisFocussed true))
    (else
      ;[1 1 1] On AI Not Focus by Character
      (if (Variables|Focus|GetisFocussed)
        (Rendering|SetVisibility (Variables|Default|GetFocusIndicator) false false)
        (Variables|Focus|SetisFocussed false)
        (Variables|Focus|SetstartFocus false)))))