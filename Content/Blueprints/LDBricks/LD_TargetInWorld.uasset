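; LD_TargetInWorld is a level-design target that the player breaks with a dash hit and that respawns afterwards.
; A timeline played from Tick animates the mesh scale.
; When a dash-hitting player capsule overlaps the mesh, it stops the dash, plays glass-break effects, disables itself, then spawns a replacement after a delay and destroys itself.
; HighLightTarget swaps materials, but its hardcoded false condition means it only ever restores the original.
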(event OnComponentBeginOverlap(Mesh)
  (params (OverlappedComponent :type Primitive%20Component%20Object%20Reference) (OtherActor :type Actor%20Object%20Reference) (OtherComp :type Primitive%20Component%20Object%20Reference) (OtherBodyIndex :type Integer) (bFromSweep :type Boolean) (SweepResult :type Hit%20Result%20Structure%20%28by%20ref%29))
  (bind _mesh (Variables|Default|GetMesh))
  (bind _ascharacter_player (Utilities|Casting|CastToCharacter_Player OtherActor))
  (if (and (== OtherComp (Variables|/Script/Engine.Character|GetCapsuleComponent _ascharacter_player)) (Utilities|Enum|Equal(Enum) (Variables|/Script/BrawlSlash.Character_Base|Getstate _ascharacter_player) "DASHING_HIT"))
    (Class|CharacterPlayer|StopDashHit _ascharacter_player)
    (Niagara|SpawnSystematLocation "/Game/Assets/VisualEffects/LD/NS_GlassBroken.NS_GlassBroken" (Transformation|GetWorldLocation (Variables|Default|GetMesh)) "0, 0, 0" "1.000000,1.000000,1.000000" false)
    (Audio|PlaySound2D 0 1.0 1.0 0.0 0 0)
    (Rendering|SetVisibility _mesh false true)
    (Collision|SetCollisionEnabled _mesh "NoCollision")
    (Collision|SetCollisionEnabled (Variables|Default|GetSphere) "NoCollision")
    (Utilities|FlowControl|Delay 2.0)
    (Game|SpawnActorfromClass "LD_TargetInWorld_C" (Math|Conversions|ToTransform(Vector) (Transformation|GetActorLocation)) "Undefined" 0 0)
    (Actor|DestroyActor)))

(event EventBeginPlay
  ;[1 1 1] Get Initials Values
  (bind _ascharacter_player (Utilities|Casting|CastToCharacter_Player (Game|GetPlayerCharacter 0)))
  (Variables|Player|Setplayer _ascharacter_player)
  (Variables|MaterialManagment|SetoldMaterial (Rendering|Material|GetMaterial (Variables|Default|GetMesh) 0)))

(event EventTick
  (params (DeltaSeconds :type Float%20%28single-precision%29))
  (if (Utilities|IsValid (Variables|Default|GetMesh))
    (bind _scale (Timeline|Scale Play)
      (:Update
        (Transformation|SetWorldScale3D (Variables|Default|GetMesh) _scale)))))

(fn ConstructionScript)

(fn HighLightTarget
  (if false
    (if (not (Variables|Target|GetisHiglighted))
      (Rendering|Material|SetMaterial (Variables|Default|GetMesh) 0 "/Game/Assets/Materials/LDBricks/M_LDBricks_IsTarget_Inst.M_LDBricks_IsTarget_Inst")
      (Variables|Target|SetisHiglighted true))
    (elif (Variables|Target|GetisHiglighted)
      (Rendering|Material|SetMaterial (Variables|Default|GetMesh) 0 (Variables|MaterialManagment|GetoldMaterial))
      (Variables|Target|SetisHiglighted false))))