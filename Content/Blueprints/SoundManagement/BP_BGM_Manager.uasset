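; BP_BGM_Manager switches background music between a navigation track and a fight track based on the player's combat state.
; On BeginPlay it caches the player character and marks the navigation song as playing.
; Each Tick it polls the player's IsInFight flag and, using a boolean to act only on changes, stops one audio component and restarts the other from the beginning.
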(event EventBeginPlay
  (bind _ascharacter_player (Utilities|Casting|CastToCharacter_Player (Game|GetPlayerCharacter 0)))
  (Variables|Default|Setplayer _ascharacter_player)
  (Variables|Default|SetisPlayingNavSong true))

(event EventTick
  (params (DeltaSeconds :type Float%20%28single-precision%29))
  (if (Variables|/Script/BrawlSlash.Character_Base|GetisInFight (Variables|Default|GetPlayer))
    (if (Variables|Default|GetisPlayingNavSong)
      (Audio|Components|Audio|Stop (Variables|Default|GetBGM_Navigation))
      (Audio|Components|Audio|Play (Variables|Default|GetBGM_FIght) 0.0)
      (Variables|Default|SetisPlayingNavSong false))
    (elif (not (Variables|Default|GetisPlayingNavSong))
      (Audio|Components|Audio|Stop (Variables|Default|GetBGM_FIght))
      (Audio|Components|Audio|Play (Variables|Default|GetBGM_Navigation) 0.0)
      (Variables|Default|SetisPlayingNavSong true))))

(fn ConstructionScript)